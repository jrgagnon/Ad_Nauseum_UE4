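; Slimey is the player's Paper2D side-scroller slime character, with shooting, jumping, wall kicks and a swap to a Mini pawn.
; Holding fire tints the sprite and builds a charge that selects a red bullet over green or plasma-upgraded blue.
; A state enum drives flipbooks, while tile-map overlaps enable wall jumps.
; It also loads or creates the save, creates the HUD, takes enemy bullet damage and opens pause and death menus.
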(event OnComponentBeginOverlap(WallCheck)
  (params (OverlappedComponent :type Primitive%20Component%20Object%20Reference) (OtherActor :type Actor%20Object%20Reference) (OtherComp :type Primitive%20Component%20Object%20Reference) (OtherBodyIndex :type Integer) (bFromSweep :type Boolean) (SweepResult :type Hit%20Result%20Structure%20%28by%20ref%29))
  ;[1 1 1] Check If Touching Wall
  (Utilities|Casting|CastToPaperTileMapActor OtherActor)
  (Variables|States|SettouchingWall true))

(event OnComponentEndOverlap(WallCheck)
  (params (OverlappedComponent :type Primitive%20Component%20Object%20Reference) (OtherActor :type Actor%20Object%20Reference) (OtherComp :type Primitive%20Component%20Object%20Reference) (OtherBodyIndex :type Integer))
  ;[1 1 1] Change var after im not touching wall
  (Utilities|Casting|CastToPaperTileMapActor OtherActor)
  (Variables|States|SettouchingWall false))

(event Custom|Restart%20the%20Level
  ;[1 1 1] Restarts Level
  (bind _returnvalue (Game|GetCurrentLevelName true))
  (Game|OpenLevel(byName) (Utilities|String|StringToName _returnvalue)))

(event Custom|UpdateAnimation
  (bind _sprite (Variables|Default|GetSprite))
  (bind _sprite_2 (Variables|Default|GetSprite))
  ;[1 1 1] Handle Animations
  (switch Utilities|FlowControl|Switch|SwitchonSlimeyStates (Variables|States|Getstates)
    (:NewEnumerator1
      (Sprite|SetFlipbook _sprite (select (> (Math|Vector|VectorLength (Transformation|GetVelocity)) 0.0) "/Game/Ad_Nauseum/Flipbooks/SlimeyMove.SlimeyMove" "/Game/Ad_Nauseum/Flipbooks/SlimeyIdle.SlimeyIdle")))
    (:NewEnumerator0
      (Sprite|SetFlipbook _sprite "/Game/Ad_Nauseum/Flipbooks/SlimeyIdle.SlimeyIdle"))
    (:NewEnumerator5
      (Sprite|SetFlipbook _sprite "/Game/Ad_Nauseum/Flipbooks/SlimeyJump.SlimeyJump"))
    (:NewEnumerator2
      (Sprite|SetFlipbook _sprite "/Game/Ad_Nauseum/Flipbooks/SlimeyShoot.SlimeyShoot"))
    (:NewEnumerator3
      (Sprite|SetFlipbook _sprite_2 "/Game/Ad_Nauseum/Flipbooks/SlimeyDie.SlimeyDie")
      (Components|Timeline|SetLooping _sprite_2 false))))

(event Custom|Update%20Powerups
  ;[1 1 1] Update Powerups
  (Variables|Default|SetplasmaShot true))

(event Custom|Update%20Health
  (params (Damage%20In :type Float%20%28single-precision%29))
  ;[1 1 1] Health System
  (if (> (- (Variables|Health|GetcurrentHealth) Damage%20In) (Variables|Health|GetmaxHealth))
    ;;[1 1 1] If I pickup more health than max set to max
    (Variables|Health|SetcurrentHealth (Variables|Health|GetmaxHealth))
    (else
      (bind _output_get (Variables|Health|SetcurrentHealth (- (Variables|Health|GetcurrentHealth) Damage%20In)))
      (if (<= _output_get 0.0)
        (Variables|States|Setstates "NewEnumerator3")
        (Variables|States|SetisDead true)
        (CallFunction|ImDead)))))

(event Custom|ImDead
  ;[1 1 1] Handle Death
  (Input|DisableInput 0)
  (Utilities|FlowControl|Delay 1.0)
  (if false
    (Viewport|RemoveAllWidgets)
    (bind _returnvalue (UserInterface|CreateWidget "/Game/Ad_Nauseum/MenuItems/OutOfLivesDS.OutOfLivesDS_C"))
    (UserInterface|Viewport|AddtoViewport _returnvalue 0)
    (Variables|/Script/Engine.PlayerController|SetbShowMouseCursor (Game|GetPlayerController 0) true)
    (else
      (Viewport|RemoveAllWidgets)
      (bind _returnvalue_2 (UserInterface|CreateWidget "/Game/Ad_Nauseum/MenuItems/DeathScreen.DeathScreen_C"))
      (UserInterface|Viewport|AddtoViewport _returnvalue_2 0)
      (Variables|/Script/Engine.PlayerController|SetbShowMouseCursor (Game|GetPlayerController 0) true))))

(event EventTick
  (params (DeltaSeconds :type Float%20%28single-precision%29))
  ;[1 1 1] Tick - Updates animation
  (CallFunction|UpdateAnimation)
  (Math|Float|CompareFloat (.X (Math|Vector|BreakVector (Variables|/Script/Engine.MovementComponent|GetVelocity (Pawn|GetMovementComponent)))) 0.0
    (:>
      (Pawn|SetControlRotation (Pawn|GetController) (Math|Rotator|MakeRotator 0.0 0.0 0.0) :!label _label))
    (:==
      (if (Variables|States|GetbisMovingRight)
        (goto _label)
        (else
          (Pawn|SetControlRotation (Pawn|GetController) (Math|Rotator|MakeRotator 0.0 0.0 1.8e+02) :!label _label_2))))
    (:<
      (goto _label_2))))

(event Collision|EventActorBeginOverlap
  (params (OtherActor :type Actor%20Object%20Reference))
  ;[1 1 1] If I am hit by an enemy bullet damage me
  (if (Utilities|ClassIsChildOf (Utilities|GetClass OtherActor) "/Game/Ad_Nauseum/Blueprints/General/BulletGeneral.BulletGeneral_C")
    (bind _asbullet_general (Utilities|Casting|CastToBulletGeneral OtherActor))
    (if (Variables|/Game/Ad_Nauseum/Blueprints/General/BulletGeneral.BulletGeneral_C|GetenemyBullet _asbullet_general)
      (CallFunction|UpdateHealth (Variables|/Game/Ad_Nauseum/Blueprints/General/BulletGeneral.BulletGeneral_C|Getdamage _asbullet_general)))))

(event EventBeginPlay
  ;[1 1 1] Startup
  (Utilities|FlowControl|Sequence
    (:then_0
      ;[1 1 1] Load/Create Save Game
      (bind _returnvalue (SaveGame|DoesSaveGameExist "Ad_Nauseum_1" :!label _label))
      (if _returnvalue
        (bind _returnvalue_2 (SaveGame|LoadGamefromSlot "Ad_Nauseum_1"))
        (bind _output_get (Variables|SaveGame|SetSaveGameConnection _returnvalue_2))
        (bind _asad_nauseum_save (Utilities|Casting|CastToAd_Nauseum_Save _output_get))
        (Utilities|FlowControl|Sequence
          (:then_0
            (Variables|SaveGame|SetS_levelCompleted (Variables|/Game/Ad_Nauseum/Blueprints/General/Ad_Nauseum_Save.Ad_Nauseum_Save_C|GetlevelCompleted _asad_nauseum_save)))
          (:then_1
            (Variables|SaveGame|SetS_levelUnlocked (Variables|/Game/Ad_Nauseum/Blueprints/General/Ad_Nauseum_Save.Ad_Nauseum_Save_C|GetlevelUnlocked _asad_nauseum_save)))
          (:then_2
            (Variables|SaveGame|SetS_levelIndexForMenu (Variables|/Game/Ad_Nauseum/Blueprints/General/Ad_Nauseum_Save.Ad_Nauseum_Save_C|GetlevelIndexForMenu _asad_nauseum_save)))
          (:then_3
            (Variables|SaveGame|SetS_levelName (Variables|/Game/Ad_Nauseum/Blueprints/General/Ad_Nauseum_Save.Ad_Nauseum_Save_C|GetlevelName _asad_nauseum_save))))
        (else
          (bind _returnvalue_3 (SaveGame|CreateSaveGameObject "/Game/Ad_Nauseum/Blueprints/General/Ad_Nauseum_Save.Ad_Nauseum_Save_C"))
          (bind _output_get_2 (Variables|SaveGame|SetSaveGameConnection _returnvalue_3))
          (bind _asad_nauseum_save_2 (Utilities|Casting|CastToAd_Nauseum_Save _output_get_2))
          (SaveGame|SaveGametoSlot _asad_nauseum_save_2 "Ad_Nauseum_1")
          (goto _label))))
    (:then_1
      (Class|ActorComponent|SetIsReplicated (Variables|Default|GetSprite) true))
    (:then_2
      (bind _returnvalue_4 (UserInterface|CreateWidget "/Game/Ad_Nauseum/Blueprints/General/HUD.HUD_C" (Game|GetPlayerController 0)))
      (bind _output_get_3 (Variables|Health|SethealthBar _returnvalue_4))
      (UserInterface|Viewport|AddtoViewport _output_get_3 0))
    (:then_3
      ;[1 1 1] Set my current health to max
      (Variables|Health|SetcurrentHealth (Variables|Health|GetmaxHealth)))
    (:then_4
      (Variables|/Script/Engine.CharacterMovementComponent|SetJumpZVelocity (Variables|Character|GetCharacterMovement self) (Variables|States|GetjumpZ)))))

(event EventOnLanded
  (params (Hit :type Hit%20Result%20Structure%20%28by%20ref%29))
  ;[1 1 1] Jump/WallJump
  (Variables|States|SetinAir false)
  (Variables|States|SettouchingWall false))

(event Input|ActionEvents|InputActionShoot
  (params (Key :type Key%20Structure :default "AnyKey"))
  ;[1 1 1] Regular and Charge Shot
  (:Pressed
    (Utilities|FlowControl|Sequence
      (:then_0
        ;[1 1 1] Change Color to Indicate Charge
        (bind _color (Timeline|Color PlayFromStart)
          (:Update
            (Sprite|SetSpriteColor (Variables|Default|GetSprite self) (Utilities|Struct|MakeLinearColor 1.0 _color _color 1.0)))))
      (:then_1
        (Timeline|Charge PlayFromStart
          (:Charge
            (Variables|States|SetshotCharge (+ (Variables|States|GetshotCharge) 1.0)))))))
  (:Released
    (Variables|States|Setstates "NewEnumerator2")
    (CallFunction|UpdateAnimation)
    (Utilities|FlowControl|Sequence
      (:then_0
        (Timeline|Color Stop))
      (:then_1
        (Timeline|Charge Stop))
      (:then_2
        (if (>= (Variables|States|GetshotCharge) (Variables|States|GetmaxChargeTime))
          (Variables|States|SetshotCharge 0.0)
          (Game|SpawnActorfromClass "/Game/Ad_Nauseum/Blueprints/Weapons/RedBullet.RedBullet_C" (Transformation|GetWorldTransform (Variables|Default|GetShootPoint)) "AlwaysSpawn" 0 0)
          (Audio|PlaySound2D "/Game/Ad_Nauseum/Sounds/slime_projectile_2.slime_projectile_2")
          (else
            (Variables|States|SetshotCharge 0.0)
            (if (Variables|Default|GetplasmaShot)
              (Game|SpawnActorfromClass "/Game/Ad_Nauseum/Blueprints/Weapons/BlueBullet.BlueBullet_C" (Transformation|GetWorldTransform (Variables|Default|GetShootPoint)) "AlwaysSpawn" 0 0)
              (else
                (Game|SpawnActorfromClass "/Game/Ad_Nauseum/Blueprints/Weapons/GreenBullet.GreenBullet_C" (Transformation|GetWorldTransform (Variables|Default|GetShootPoint)) "AlwaysSpawn" 0 0)))
            (Audio|PlaySound2D "/Game/Ad_Nauseum/Sounds/slime_projectile_2.slime_projectile_2")))
        (Utilities|FlowControl|Delay 0.3)
        (Variables|States|Setstates "NewEnumerator0")
        (CallFunction|UpdateAnimation))
      (:then_3
        (Sprite|SetSpriteColor (Variables|Default|GetSprite self) "(R=1.000000,G=1.000000,B=1.000000,A=1.000000)")))))

(event Input|ActionEvents|InputActionPGame
  (params (Key :type Key%20Structure :default "AnyKey"))
  ;[1 1 1] Pause Game, Load Pause Menu
  (:Pressed
    (Game|SetGamePaused true)
    (Viewport|RemoveAllWidgets)
    (bind _returnvalue (UserInterface|CreateWidget "/Game/Ad_Nauseum/MenuItems/PauseMenu.PauseMenu_C"))
    (UserInterface|Viewport|AddtoViewport _returnvalue 0)
    (Variables|/Script/Engine.PlayerController|SetbShowMouseCursor (Game|GetPlayerController 0) true)))

(event Input|ActionEvents|InputActionJump
  (params (Key :type Key%20Structure :default "AnyKey"))
  ;[1 1 1] Jump/WallJump
  (:Pressed
    (if (and (Variables|States|GettouchingWall) (Variables|States|GetinAir))
      (if (Variables|States|GetbisMovingRight)
        (Variables|States|SetwallKickMultiplier -1.0)
        (else
          (Variables|States|SetwallKickMultiplier 1.0)))
      (Character|LaunchCharacter (Math|Vector|MakeVector (* (Variables|States|GetjumpZ) (Variables|States|GetwallKickMultiplier)) 0.0 (.Z (Math|Vector|BreakVector (* (Transformation|GetActorUpVector) (Variables|States|GetjumpZ))))) false false)
      (Variables|States|Setstates "NewEnumerator5")
      (Variables|States|SettouchingWall false)
      (else
        (Character|Jump)
        (Variables|States|Setstates "NewEnumerator5")
        (Variables|States|SetinAir true))))
  (:Released
    (Character|StopJumping)
    (Utilities|FlowControl|Delay 0.2)
    (Variables|States|Setstates "NewEnumerator0")))

(event Input|AxisEvents|InputAxisMoveRight
  (params (AxisValue :type Float%20%28single-precision%29))
  ;[1 1 1] Handle Movement
  (if (> AxisValue 0.0)
    (Variables|States|SetbisMovingRight true)
    (elif (< AxisValue 0.0)
      (Variables|States|SetbisMovingRight false)))
  (Pawn|Input|AddMovementInput "1.000000, 0, 0" AxisValue false)
  (if (not (Variables|States|GetisJumping))
    (if (not (Variables|States|GetisDead))
      (Variables|States|Setstates "NewEnumerator1"))))

(event Input|KeyboardEvents|Slash
  (params (Key :type Key%20Structure :default "AnyKey"))
  ;[1 1 1] Debug Health
  (:Pressed
    (CallFunction|UpdateHealth 1e+02)))

(event Input|KeyboardEvents|M
  (params (Key :type Key%20Structure :default "AnyKey"))
  ;[1 1 1] Mini Form
  (:Pressed
    (Pawn|UnPossess (Game|GetPlayerController 0))
    (Actor|DestroyActor)
    (bind _returnvalue (Game|SpawnActorfromClass "/Game/Ad_Nauseum/Blueprints/General/Mini.Mini_C" (Transformation|GetActorTransform) "Undefined" 0 0))
    (Pawn|Possess (Game|GetPlayerController 0) _returnvalue)))

(event Input|KeyboardEvents|Backslash
  (params (Key :type Key%20Structure :default "AnyKey"))
  ;[1 1 1] Debug Level Restart
  (:Pressed
    (CallFunction|RestarttheLevel)))

(fn ConstructionScript)