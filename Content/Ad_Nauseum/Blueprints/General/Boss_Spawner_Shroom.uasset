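; Trigger actor that spawns a boss, presumably the Shroom boss, when Slimey enters its SpawnTrigger volume.
; On the first such overlap it widens Slimey's orthographic side-view camera to frame the fight.
; It then spawns the BossToSpawn class, scaled up sevenfold, at an offset from its root, and sets a Spawned flag so later overlaps do nothing.
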(event OnComponentBeginOverlap(SpawnTrigger)
  (params (OverlappedComponent :type Primitive%20Component%20Object%20Reference) (OtherActor :type Actor%20Object%20Reference) (OtherComp :type Primitive%20Component%20Object%20Reference) (OtherBodyIndex :type Integer) (bFromSweep :type Boolean) (SweepResult :type Hit%20Result%20Structure%20%28by%20ref%29))
  (bind _asslimey (Utilities|Casting|CastToSlimey OtherActor))
  (if (not (Variables|Default|Getspawned))
    (Class|CameraComponent|SetOrthoWidth (Variables|/Game/Ad_Nauseum/Blueprints/General/Slimey.Slimey_C|GetSideViewCameraComponent _asslimey) 2e+03)
    (Game|SpawnActorfromClass (Variables|Default|GetbossToSpawn) (Math|Transform|MakeTransform (+ (Transformation|GetWorldLocation (Variables|Default|GetRoot)) (Variables|Default|GetlocationToSpawn)) "0, 0, 0" "7.000000,7.000000,7.000000") "Undefined" 0 0)
    (Variables|Default|Setspawned true)))

(event EventBeginPlay)

(event Collision|EventActorBeginOverlap
  (params (OtherActor :type Actor%20Object%20Reference)))

(event EventTick
  (params (DeltaSeconds :type Float%20%28single-precision%29)))

(fn ConstructionScript)