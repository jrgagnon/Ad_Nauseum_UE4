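; BlueBullet is a weapon projectile actor that destroys itself five seconds after it spawns.
; On overlap, a chain of casts ignores the ZacBossspooner and Slimey classes.
; Tile maps, breaking platforms and both moving platform types make it destroy itself after a very short delay.
; The graph contains no movement or damage logic.
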(event EventBeginPlay
  (Utilities|FlowControl|Delay 5.0)
  (Actor|DestroyActor))

(event Collision|EventActorBeginOverlap
  (params (OtherActor :type Actor%20Object%20Reference))
  (Utilities|Casting|CastToZacBossspooner OtherActor
    (:CastFailed
      (Utilities|Casting|CastToSlimey OtherActor
        (:CastFailed
          (Utilities|Casting|CastToPaperTileMapActor OtherActor
            (:then
              _)
            (:CastFailed
              (Utilities|Casting|CastToBreaking_Platform OtherActor
                (:then
                  _)
                (:CastFailed
                  (Utilities|Casting|CastToMoving_Platform OtherActor
                    (:then
                      _)
                    (:CastFailed
                      (Utilities|Casting|CastToMoving_Platform2 OtherActor)))))))
          (Utilities|FlowControl|Delay 0.01)
          (Actor|DestroyActor))))))

(event EventTick
  (params (DeltaSeconds :type Float%20%28single-precision%29)))

(fn ConstructionScript
  (|CallParentFunction))