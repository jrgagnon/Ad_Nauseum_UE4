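; Coal bomb projectile for the snowman boss, built on a physics-driven Paper2D sprite that explodes on contact.
; Shortly after BeginPlay it gets a single horizontal force, with the Direction flag choosing the sign.
; On overlap, a chain of casts ignores the boss spawner class ZacBossspooner, the snowman's middle, explosions and general bullets.
; Any other actor makes it spawn an Explosion at its transform and destroy itself.
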(event EventBeginPlay
  (bind _force (Variables|Default|GetForce))
  (Utilities|FlowControl|Delay 0.2)
  (if (Variables|Default|GetDirection)
    (Physics|AddForce (Variables|Default|GetPaperSprite) (Math|Vector|MakeVector _force 0.0 0.0) "None" false)
    (else
      (Physics|AddForce (Variables|Default|GetPaperSprite) (Math|Vector|MakeVector (* -1.0 _force) 0.0 0.0) "None" false))))

(event Collision|EventActorBeginOverlap
  (params (OtherActor :type Actor%20Object%20Reference))
  (Utilities|Casting|CastToZacBossspooner OtherActor
    (:CastFailed
      (Utilities|Casting|CastToSnowmanBossMiddle OtherActor
        (:CastFailed
          (Utilities|Casting|CastToExplosion OtherActor
            (:CastFailed
              (Utilities|Casting|CastToBulletGeneral OtherActor
                (:CastFailed
                  (Game|SpawnActorfromClass "/Game/Ad_Nauseum/Blueprints/Weapons/Explosion.Explosion_C" (Transformation|GetActorTransform) "Undefined" 0 0)
                  (Actor|DestroyActor))))))))))

(event EventTick
  (params (DeltaSeconds :type Float%20%28single-precision%29)))

(fn ConstructionScript)