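; Mushroom boss enemy that repeatedly force-jumps on a delay and rains Falling_B actors between its posts when it lands.
; Landing is detected by overlapping a BossFloorTrigger after a jump, which plays a footstep sound and zeroes velocity.
; Ping-pong timeline events handle patrol between LeftPost and RightPost, though BeginPlay only sets their play rate.
; Sprite overlaps also damage Slimey or apply player bullet damage, destroying the boss at zero health.
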(event OnComponentBeginOverlap(PaperSprite)
  (params (OverlappedComponent :type Primitive%20Component%20Object%20Reference) (OtherActor :type Actor%20Object%20Reference) (OtherComp :type Primitive%20Component%20Object%20Reference) (OtherBodyIndex :type Integer) (bFromSweep :type Boolean) (SweepResult :type Hit%20Result%20Structure%20%28by%20ref%29))
  (bind _leftpost (Variables|Default|GetLeftPost))
  ;[1 1 1] Actor Overlap Handling
  ;;[1 1 1] If Slimey is Hit Damage Him
  (bind _asslimey (Utilities|Casting|CastToSlimey OtherActor)
    (:then
      (Default|UpdateHealth _asslimey 25.0))
    (:CastFailed
      ;;[1 1 1] If I am hit determine damage, then damage me
      (if (Utilities|ClassIsChildOf (Utilities|GetClass OtherActor) "/Game/Ad_Nauseum/Blueprints/General/BulletGeneral.BulletGeneral_C")
        (bind _asbullet_general (Utilities|Casting|CastToBulletGeneral OtherActor))
        (if (not (Variables|/Game/Ad_Nauseum/Blueprints/General/BulletGeneral.BulletGeneral_C|GetenemyBullet _asbullet_general))
          (Audio|SpawnSound2D "/Game/Ad_Nauseum/Sounds/slime_impact_5.slime_impact_5")
          (CallFunction|PatrolHit (Variables|/Game/Ad_Nauseum/Blueprints/General/BulletGeneral.BulletGeneral_C|Getdamage _asbullet_general)))
        (else
          (Utilities|Casting|CastToBossFloorTrigger OtherActor)
          (if (Variables|Default|GetJumped)
            (Audio|PlaySound2D "/Game/Ad_Nauseum/Sounds/mushroom_boss_footstep.mushroom_boss_footstep" 2.0)
            (Variables|Default|SetJumped false)
            (Physics|SetPhysicsLinearVelocity (Variables|Default|GetPaperSprite) "0, 0, 0" false "None")
            (for _index (range 0 7)
              (Game|SpawnActorfromClass "/Game/Ad_Nauseum/Blueprints/Traps/Falling_B.Falling_B_C" (Math|Transform|MakeTransform (Math|Vector|MakeVector (+ (* (Math|Random|RandomFloat) (- (Variables|Default|GetRightPost) _leftpost)) _leftpost) 0.0 1.23e+03) "0, 0, 0" "1,1,1") "Undefined" 0 0))))))))

(event Custom|BossJump
  ;[1 1 1] Boss Jump Function
  (Physics|AddForce (Variables|Default|GetPaperSprite) (Math|Vector|MakeVector 0.0 0.0 (Variables|Default|GetBossJumpForce)) "None" false)
  (Variables|Default|SetJumped true)
  (Utilities|FlowControl|Delay (Variables|Default|GetJumpDelay))
  (CallFunction|BossJump))

(event Custom|PatrolHit
  (params (DamageIn :type Float%20%28single-precision%29))
  ;[1 1 1] Damage Me
  (bind _output_get (Variables|Default|SetcurrentHealth (- (Variables|Default|GetcurrentHealth) DamageIn)))
  ;[1 1 1] Kill me if health is <= 0
  (if (<= _output_get 0.0)
    (Actor|DestroyActor)))

(event Custom|Moving%20Forward
  (bind _papersprite (Variables|Default|GetPaperSprite))
  (bind _returnvalue (Transformation|GetRelativeTransform _papersprite))
  ;[1 1 1] Handle Movement
  (bind (_direction _newtrack_0) (Timeline|PatrolTimeline PlayFromStart)
    (:Update
      (Transformation|SetRelativeLocation (Variables|Default|GetPaperSprite) (Math|Vector|MakeVector (+ (* _newtrack_0 (- (Variables|Default|GetRightPost) (Variables|Default|GetLeftPost))) (Variables|Default|GetLeftPost)) (.y (.location _returnvalue)) (.z (.location _returnvalue))) false false))
    (:Finished
      (switch Utilities|FlowControl|Switch|SwitchonETimelineDirection _direction
        (:Forward
          (CallFunction|MovingBackward))
        (:Backward
          (CallFunction|MovingForward))))))

(event Custom|Moving%20Backward
  (bind _papersprite (Variables|Default|GetPaperSprite))
  (bind _returnvalue (Transformation|GetRelativeTransform _papersprite))
  ;[1 1 1] Handle Movement
  (bind (_direction _newtrack_0) (Timeline|PatrolTimeline ReverseFromEnd)
    (:Update
      (Transformation|SetRelativeLocation (Variables|Default|GetPaperSprite) (Math|Vector|MakeVector (+ (* _newtrack_0 (- (Variables|Default|GetRightPost) (Variables|Default|GetLeftPost))) (Variables|Default|GetLeftPost)) (.y (.location _returnvalue)) (.z (.location _returnvalue))) false false))
    (:Finished
      (switch Utilities|FlowControl|Switch|SwitchonETimelineDirection _direction
        (:Forward
          (CallFunction|MovingBackward))
        (:Backward
          (CallFunction|MovingForward))))))

(event EventBeginPlay
  ;[1 1 1] On Startup
  (Utilities|FlowControl|Sequence
    (:then_0
      (Components|Timeline|SetPlayRate (Variables|Default|GetPatrolTimeline) (Variables|Default|GetMoveRate)))
    (:then_1
      (Class|PrimitiveComponent|SetMassOverrideinKg (Variables|Default|GetPaperSprite) "None" 6.0 true))
    (:then_2
      (CallFunction|BossJump))))

(event Collision|EventActorBeginOverlap
  (params (OtherActor :type Actor%20Object%20Reference)))

(event EventTick
  (params (DeltaSeconds :type Float%20%28single-precision%29)))

(fn ConstructionScript)