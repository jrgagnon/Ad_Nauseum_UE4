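; Scorpion claw Blueprint, a damageable mob part that hurts Slimey on overlap.
; It starts at max health and handles all contact in one overlap event, dealing fixed damage when the other actor is Slimey.
; When Damageable, it loses health to non-enemy BulletGeneral projectiles by their Damage value and sets a Dead flag at zero or below, with no further death handling in this Blueprint.
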(event EventBeginPlay
  ;[1 1 1] Set Current Health to max health
  (Variables|Default|SetcurrentHealth (Variables|Default|GetmaxHealth)))

(event Collision|EventActorBeginOverlap
  (params (OtherActor :type Actor%20Object%20Reference))
  ;[1 1 1] Actor Overlap Handling
  ;;[1 1 1] If Slimey is Hit Damage Him
  (bind _asslimey (Utilities|Casting|CastToSlimey OtherActor)
    (:then
      (Default|UpdateHealth _asslimey 25.0))
    (:CastFailed
      ;;[1 1 1] Check to see if i can be damaged
      (if (Utilities|ClassIsChildOf (Utilities|GetClass OtherActor) "/Game/Ad_Nauseum/Blueprints/General/BulletGeneral.BulletGeneral_C")
        (if (Variables|Default|Getdamageable)
          (bind _asbullet_general (Utilities|Casting|CastToBulletGeneral OtherActor))
          (if (not (Variables|/Game/Ad_Nauseum/Blueprints/General/BulletGeneral.BulletGeneral_C|GetenemyBullet _asbullet_general))
            (bind _output_get (Variables|Default|SetcurrentHealth (- (Variables|Default|GetcurrentHealth) (Variables|/Game/Ad_Nauseum/Blueprints/General/BulletGeneral.BulletGeneral_C|Getdamage _asbullet_general))))
            (if (<= _output_get 0.0)
              (Variables|Default|Setdead true))))))))

(fn ConstructionScript)