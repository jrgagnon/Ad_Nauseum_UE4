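; Ghost boss enemy that steadily drifts toward the player each tick and damages Slimey on overlap.
; Non-enemy bullets reduce its health; a surviving hit hides it for a second, then teleports it to a random point around its start location.
; Two teleport outcomes also summon three GhostBoss2 minions at random points; the random range reaches only five of seven points.
; On death it sometimes drops a HealthPickup.
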(event Custom|PatrolHit
  (params (DamageIn :type Float%20%28single-precision%29))
  ;[1 1 1] Damage Me
  (bind _output_get (Variables|Default|SetcurrentHealth (- (Variables|Default|GetcurrentHealth) DamageIn)))
  ;[1 1 1] Kill me if health is <= 0
  (if (<= _output_get 0.0)
    ;[1 1 1] Spawn any loot upon death
    (switch int (Math|Random|RandomIntegerinRange 0 2)
      (:0
        _)
      (:1
        (Game|SpawnActorfromClass "/Game/Ad_Nauseum/Blueprints/General/HealthPickup.HealthPickup_C" (Transformation|GetWorldTransform (Variables|Default|GetGhostBoss)) "Undefined" 0 0))
      (:2
        _))
    (Actor|DestroyActor)
    (else
      (Development|SetHiddeninGame (Variables|Default|GetRoot) true true)
      (Utilities|FlowControl|Delay 1.0)
      (CallFunction|Spawn)
      (Development|SetHiddeninGame (Variables|Default|GetGhostBoss) false false))))

(event Collision|EventActorBeginOverlap
  (params (OtherActor :type Actor%20Object%20Reference))
  ;[1 1 1] Actor Overlap Handling
  ;;[1 1 1] If Slimey is Hit Damage Him
  (bind _asslimey (Utilities|Casting|CastToSlimey OtherActor)
    (:then
      (Default|UpdateHealth _asslimey 25.0))
    (:CastFailed
      ;;[1 1 1] If I am hit determine damage, then damage me
      (if (Utilities|ClassIsChildOf (Utilities|GetClass OtherActor) "/Game/Ad_Nauseum/Blueprints/General/BulletGeneral.BulletGeneral_C")
        (bind _asbullet_general (Utilities|Casting|CastToBulletGeneral OtherActor))
        (if (not (Variables|/Game/Ad_Nauseum/Blueprints/General/BulletGeneral.BulletGeneral_C|GetenemyBullet _asbullet_general))
          (CallFunction|PatrolHit (Variables|/Game/Ad_Nauseum/Blueprints/General/BulletGeneral.BulletGeneral_C|Getdamage _asbullet_general)))))))

(event EventBeginPlay
  ;[1 1 1] Startup
  (Utilities|FlowControl|Sequence
    (:then_0
      ;[1 1 1] Set Current Health to Max on Start
      (Variables|Default|SetcurrentHealth (Variables|Default|GetmaxHealth))
      (Variables|Default|SetBossSpawn (Transformation|GetActorLocation)))))

(event EventTick
  (params (DeltaSeconds :type Float%20%28single-precision%29))
  (bind _returnvalue (Transformation|GetActorLocation))
  ;[1 1 1] Movement Control
  (Transformation|SetActorLocation (+ (* (* (Math|Vector|Normalize (- (Transformation|GetActorLocation (Game|Player|GetPlayerPawn 0)) _returnvalue)) DeltaSeconds) 5e+01) _returnvalue) false false))

(fn ConstructionScript
  (Transformation|SetRelativeLocation (Variables|Default|GetGhostBoss) (Math|Vector|SelectVector "0, 0, 0" "0, 0, 0" false) false false))

(fn Spawn
  (switch int (Math|Random|RandomIntegerinRange 0 4)
    (:0
      (Transformation|SetActorLocation (+ (Variables|Default|GetSpawn1) (Variables|Default|GetBossSpawn)) false true))
    (:1
      (Transformation|SetActorLocation (+ (Variables|Default|GetSpawn2) (Variables|Default|GetBossSpawn)) false true))
    (:2
      (Transformation|SetActorLocation (+ (Variables|Default|GetSpawn3) (Variables|Default|GetBossSpawn)) false true)
      (CallFunction|SpawnGhost2)
      (CallFunction|SpawnGhost2)
      (CallFunction|SpawnGhost2))
    (:3
      (Transformation|SetActorLocation (+ (Variables|Default|GetSpawn4) (Variables|Default|GetBossSpawn)) false true))
    (:4
      (Transformation|SetActorLocation (+ (Variables|Default|GetSpawn5) (Variables|Default|GetBossSpawn)) false true)
      (CallFunction|SpawnGhost2)
      (CallFunction|SpawnGhost2)
      (CallFunction|SpawnGhost2))
    (:5
      (Transformation|SetActorLocation (+ (Variables|Default|GetSpawn6) (Variables|Default|GetBossSpawn)) false true))
    (:6
      (Transformation|SetActorLocation (+ (Variables|Default|GetSpawn7) (Variables|Default|GetBossSpawn)) false true))))

(fn SpawnGhost2
  (switch int (Math|Random|RandomIntegerinRange 0 4)
    (:0
      (Game|SpawnActorfromClass "/Game/Ad_Nauseum/Blueprints/BasicMobs/GhostBoss2.GhostBoss2_C" (Math|Conversions|ToTransform(Vector) (+ (Variables|Default|GetSpawn1) (Variables|Default|GetBossSpawn))) "Undefined" 0 0))
    (:1
      (Game|SpawnActorfromClass "/Game/Ad_Nauseum/Blueprints/BasicMobs/GhostBoss2.GhostBoss2_C" (Math|Conversions|ToTransform(Vector) (+ (Variables|Default|GetSpawn2) (Variables|Default|GetBossSpawn))) "Undefined" 0 0))
    (:2
      (Game|SpawnActorfromClass "/Game/Ad_Nauseum/Blueprints/BasicMobs/GhostBoss2.GhostBoss2_C" (Math|Conversions|ToTransform(Vector) (+ (Variables|Default|GetSpawn3) (Variables|Default|GetBossSpawn))) "Undefined" 0 0))
    (:3
      (Game|SpawnActorfromClass "/Game/Ad_Nauseum/Blueprints/BasicMobs/GhostBoss2.GhostBoss2_C" (Math|Conversions|ToTransform(Vector) (+ (Variables|Default|GetSpawn4) (Variables|Default|GetBossSpawn))) "Undefined" 0 0))
    (:4
      (Game|SpawnActorfromClass "/Game/Ad_Nauseum/Blueprints/BasicMobs/GhostBoss2.GhostBoss2_C" (Math|Conversions|ToTransform(Vector) (+ (Variables|Default|GetSpawn5) (Variables|Default|GetBossSpawn))) "Undefined" 0 0))
    (:5
      (Game|SpawnActorfromClass "/Game/Ad_Nauseum/Blueprints/BasicMobs/GhostBoss2.GhostBoss2_C" (Math|Conversions|ToTransform(Vector) (+ (Variables|Default|GetSpawn6) (Variables|Default|GetBossSpawn))) "Undefined" 0 0))
    (:6
      (Game|SpawnActorfromClass "/Game/Ad_Nauseum/Blueprints/BasicMobs/GhostBoss2.GhostBoss2_C" (Math|Conversions|ToTransform(Vector) (+ (Variables|Default|GetSpawn7) (Variables|Default|GetBossSpawn))) "Undefined" 0 0))))