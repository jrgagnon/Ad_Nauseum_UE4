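; Scorpion boss that spawns a stinger and four tail segments as separate actors and shows its health on a BossHUD widget.
; Tick polls their Dead flags to enforce kill order: stinger, then segments, then body, each lost part also damaging the boss.
; Player bullets hurt the body once exposed, overlapping Slimey passes a fixed value to UpdateHealth, and death may drop a health pickup.
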(event Custom|ScorpionHit
  (params (DamageIn :type Float%20%28single-precision%29))
  ;[1 1 1] Damage Me
  (bind _output_get (Variables|Health|SetcurrentHealth (- (Variables|Health|GetcurrentHealth) DamageIn)))
  ;[1 1 1] Update Health Bar
  (Progress|SetPercent (Variables|/Game/Ad_Nauseum/Blueprints/General/BossHUD.BossHUD_C|GetScorpionHealth (Variables|Health|GetbossHealth)) (/ _output_get (Variables|Health|GetmaxHealth)))
  ;[1 1 1] Kill me if health is <= 0
  (if (<= _output_get 0.0)
    (Utilities|FlowControl|Sequence
      (:then_0
        ;[1 1 1] Scorpion Dead Remove His Healthbar
        (Widget|RemovefromParent (Variables|Health|GetbossHealth)))
      (:then_1
        ;[1 1 1] Spawn any loot upon death
        (switch int (Math|Random|RandomIntegerinRange 0 2)
          (:0
            _)
          (:1
            (Game|SpawnActorfromClass "/Game/Ad_Nauseum/Blueprints/General/HealthPickup.HealthPickup_C" (Transformation|GetWorldTransform (Variables|Default|GetScorpion_Body)) "Undefined" 0 0))
          (:2
            _))
        (Actor|DestroyActor)))))

(event EventBeginPlay
  (bind _maxhealth (Variables|Health|GetmaxHealth))
  ;[1 1 1] Init
  (Utilities|FlowControl|Sequence
    (:then_0
      ;;[1 1 1] Add Scorpion Healthbar to Viewport
      (bind _returnvalue (UserInterface|CreateWidget "/Game/Ad_Nauseum/Blueprints/General/BossHUD.BossHUD_C"))
      (bind _output_get (Variables|Health|SetbossHealth _returnvalue))
      (UserInterface|Viewport|AddtoViewport _output_get 0))
    (:then_1
      ;;[1 1 1] initialize Health and Health bar
      (bind _output_get_2 (Variables|Health|SetcurrentHealth _maxhealth))
      (Progress|SetPercent (Variables|/Game/Ad_Nauseum/Blueprints/General/BossHUD.BossHUD_C|GetScorpionHealth (Variables|Health|GetbossHealth)) (/ _output_get_2 _maxhealth)))
    (:then_2
      ;;[1 1 1] Set the location of the Scorpions Body
      (Variables|Locations|SetbodyLocation (Transformation|GetWorldLocation (Variables|Default|GetRoot))))
    (:then_3
      ;;[1 1 1] Spawn Tail Segments
      (bind _returnvalue_2 (Game|SpawnActorfromClass "/Game/Ad_Nauseum/Blueprints/BasicMobs/Scorpion_Tail_Segment.Scorpion_Tail_Segment_C" (Math|Transform|MakeTransform (+ (Variables|Locations|GetbodyLocation) (Variables|Locations|GettailSeg1Location)) "0, 0, 0" "1,1,1") "Undefined" 0 0))
      (Variables|Tail|SettailSeg1 _returnvalue_2)
      (bind _returnvalue_3 (Game|SpawnActorfromClass "/Game/Ad_Nauseum/Blueprints/BasicMobs/Scorpion_Tail_Segment.Scorpion_Tail_Segment_C" (Math|Transform|MakeTransform (+ (Variables|Locations|GetbodyLocation) (Variables|Locations|GettailSeg2Location)) "0, 0, 0" "1,1,1") "Undefined" 0 0))
      (Variables|Tail|SettailSeg2 _returnvalue_3)
      (bind _returnvalue_4 (Game|SpawnActorfromClass "/Game/Ad_Nauseum/Blueprints/BasicMobs/Scorpion_Tail_Segment.Scorpion_Tail_Segment_C" (Math|Transform|MakeTransform (+ (Variables|Locations|GetbodyLocation) (Variables|Locations|GettailSeg3Location)) "0, 0, 0" "1,1,1") "Undefined" 0 0))
      (Variables|Tail|SettailSeg3 _returnvalue_4)
      (bind _returnvalue_5 (Game|SpawnActorfromClass "/Game/Ad_Nauseum/Blueprints/BasicMobs/Scorpion_Tail_Segment.Scorpion_Tail_Segment_C" (Math|Transform|MakeTransform (+ (Variables|Locations|GetbodyLocation) (Variables|Locations|GettailSeg4Location)) "0, 0, 0" "1,1,1") "Undefined" 0 0))
      (Variables|Tail|SettailSeg4 _returnvalue_5))
    (:then_4
      ;;[1 1 1] Spawn the Stinger
      (bind _returnvalue_6 (Game|SpawnActorfromClass "/Game/Ad_Nauseum/Blueprints/BasicMobs/Scorpion_Stinger.Scorpion_Stinger_C" (Math|Transform|MakeTransform (+ (Variables|Locations|GetbodyLocation) (Variables|Locations|GetstingerLocation)) "0, 0, 0" "1,1,1") "Undefined" 0 0))
      (Variables|Tail|Setstinger _returnvalue_6))))

(event Collision|EventActorBeginOverlap
  (params (OtherActor :type Actor%20Object%20Reference))
  ;[1 1 1] Actor Overlap Handling
  ;;[1 1 1] If Slimey is Hit Damage Him
  (bind _asslimey (Utilities|Casting|CastToSlimey OtherActor)
    (:then
      (Default|UpdateHealth _asslimey 25.0))
    (:CastFailed
      ;;[1 1 1] If I am hit determine damage, then damage me
      (if (Utilities|ClassIsChildOf (Utilities|GetClass OtherActor) "/Game/Ad_Nauseum/Blueprints/General/BulletGeneral.BulletGeneral_C")
        (bind _asbullet_general (Utilities|Casting|CastToBulletGeneral OtherActor))
        (if (not (Variables|/Game/Ad_Nauseum/Blueprints/General/BulletGeneral.BulletGeneral_C|GetenemyBullet _asbullet_general))
          (if (Variables|Booleans|GetbodyDamageable)
            (CallFunction|ScorpionHit (Variables|/Game/Ad_Nauseum/Blueprints/General/BulletGeneral.BulletGeneral_C|Getdamage _asbullet_general))))))))

(event EventTick
  (params (DeltaSeconds :type Float%20%28single-precision%29))
  (bind _tailseg1 (Variables|Tail|GettailSeg1))
  (bind _stinger (Variables|Tail|Getstinger))
  (bind _tailseg2 (Variables|Tail|GettailSeg2))
  (bind _tailseg3 (Variables|Tail|GettailSeg3))
  (bind _tailseg4 (Variables|Tail|GettailSeg4))
  ;[1 1 1] On Tick
  (if (Variables|Booleans|GetstingerDead)
    (if (not (Variables|Booleans|GetsegmentsDead))
      (Utilities|FlowControl|Sequence
        (:then_0
          ;;[1 1 1] Check Seg1 Status
          (if (not (Variables|Booleans|Getseg1Dead))
            (if (Variables|/Game/Ad_Nauseum/Blueprints/BasicMobs/Scorpion_Tail_Segment.Scorpion_Tail_Segment_C|Getdead _tailseg1)
              (Actor|DestroyActor _tailseg1)
              (Variables|Booleans|Setseg1Dead true)
              (CallFunction|ScorpionHit 25.0))))
        (:then_1
          ;;[1 1 1] Check Seg2 Status
          (if (not (Variables|Booleans|Getseg2Dead))
            (if (Variables|/Game/Ad_Nauseum/Blueprints/BasicMobs/Scorpion_Tail_Segment.Scorpion_Tail_Segment_C|Getdead _tailseg2)
              (Actor|DestroyActor _tailseg2)
              (Variables|Booleans|Setseg2Dead true)
              (CallFunction|ScorpionHit 25.0))))
        (:then_2
          ;;[1 1 1] Check Seg3 Status
          (if (not (Variables|Booleans|Getseg3Dead))
            (if (Variables|/Game/Ad_Nauseum/Blueprints/BasicMobs/Scorpion_Tail_Segment.Scorpion_Tail_Segment_C|Getdead _tailseg3)
              (Actor|DestroyActor _tailseg3)
              (Variables|Booleans|Setseg3Dead true)
              (CallFunction|ScorpionHit 25.0))))
        (:then_3
          ;;[1 1 1] Check Seg4 Status
          (if (not (Variables|Booleans|Getseg4Dead))
            (if (Variables|/Game/Ad_Nauseum/Blueprints/BasicMobs/Scorpion_Tail_Segment.Scorpion_Tail_Segment_C|Getdead _tailseg4)
              (Actor|DestroyActor _tailseg4)
              (Variables|Booleans|Setseg4Dead true)
              (CallFunction|ScorpionHit 25.0))))
        (:then_4
          ;;[1 1 1] If all segments dead make body damageable
          (bind _output_get (Variables|Booleans|SetsegmentsDead (Math|Boolean|ANDBoolean (Variables|Booleans|Getseg1Dead) (Variables|Booleans|Getseg2Dead) (Variables|Booleans|Getseg3Dead) (Variables|Booleans|Getseg4Dead))))
          (Variables|Booleans|SetbodyDamageable _output_get))))
    (else
      ;;[1 1 1] Stinger is Dead Kill it make segments damageable
      (if (Variables|/Game/Ad_Nauseum/Blueprints/BasicMobs/Scorpion_Stinger.Scorpion_Stinger_C|Getdead _stinger)
        (Actor|DestroyActor _stinger)
        (Variables|/Game/Ad_Nauseum/Blueprints/BasicMobs/Scorpion_Tail_Segment.Scorpion_Tail_Segment_C|Setdamageable (Variables|Tail|GettailSeg1) true)
        (Variables|/Game/Ad_Nauseum/Blueprints/BasicMobs/Scorpion_Tail_Segment.Scorpion_Tail_Segment_C|Setdamageable (Variables|Tail|GettailSeg2) true)
        (Variables|/Game/Ad_Nauseum/Blueprints/BasicMobs/Scorpion_Tail_Segment.Scorpion_Tail_Segment_C|Setdamageable (Variables|Tail|GettailSeg3) true)
        (Variables|/Game/Ad_Nauseum/Blueprints/BasicMobs/Scorpion_Tail_Segment.Scorpion_Tail_Segment_C|Setdamageable (Variables|Tail|GettailSeg4) true)
        (Variables|Booleans|SetstingerDead true)
        (CallFunction|ScorpionHit 25.0)))))

(fn ConstructionScript)