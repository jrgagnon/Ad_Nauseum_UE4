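; Slime enemy that damages an overlapping Slimey and takes damage from non-enemy BulletGeneral projectiles.
; At zero health it destroys itself, with a one-in-three chance of spawning a HealthPickup first.
; ToFirst, not called in this graph, starts timeline-lerped movement to FirstPoint, then MovingForward cycles through four point indices with stop delays.
; The construction script previews the slime at FirstPoint or its origin via TestRightEnd.
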(event Custom|Moving%20Forward
  ;[1 1 1] Movement Control
  (bind _track (Timeline|Timeline_0 PlayFromStart)
    (:Update
      (Transformation|SetRelativeLocation (Variables|Components|GetSlime) (Math|Vector|Lerp(Vector) (Variables|Default|GetPrevious) (Utilities|Array|Get(acopy) (Utilities|Array|MakeArray (Variables|Default|GetfirstPoint) (Variables|Default|GetsecondPoint) (Variables|Default|GetthirdPoint) (Variables|Default|GetfourthPoint)) (Variables|Default|GetNext)) _track) false true))
    (:Finished
      (Utilities|FlowControl|Delay (Variables|Default|GetstopDelay))
      (if (== (Variables|Default|GetNext) 3)
        (Variables|Default|SetNext 0)
        (Variables|Default|SetPrevious (Utilities|Array|Get(acopy) (Utilities|Array|MakeArray (Variables|Default|GetfirstPoint) (Variables|Default|GetsecondPoint) (Variables|Default|GetthirdPoint) (Variables|Default|GetfourthPoint)) (Variables|Default|GetNext)))
        (else
          (Math|Integer|IncrementInt (Variables|Default|GetNext)
            (:%20%20
              (Variables|Default|SetPrevious (Utilities|Array|Get(acopy) (Utilities|Array|MakeArray (Variables|Default|GetfirstPoint) (Variables|Default|GetsecondPoint) (Variables|Default|GetthirdPoint) (Variables|Default|GetfourthPoint)) (Variables|Default|GetNext)))))))
      (CallFunction|MovingForward))))

(event Custom|PatrolHit
  (params (DamageIn :type Float%20%28single-precision%29))
  ;[1 1 1] Damage Me
  (bind _output_get (Variables|Default|SetcurrentHealth (- (Variables|Default|GetcurrentHealth) DamageIn)))
  ;[1 1 1] Kill me if health is <= 0
  (if (<= _output_get 0.0)
    ;[1 1 1] Spawn any loot upon death
    (switch int (Math|Random|RandomIntegerinRange 0 2)
      (:0
        _)
      (:1
        (Game|SpawnActorfromClass "/Game/Ad_Nauseum/Blueprints/General/HealthPickup.HealthPickup_C" (Transformation|GetWorldTransform (Variables|Components|GetSlime)) "Undefined" 0 0))
      (:2
        _))
    (Actor|DestroyActor)))

(event Custom|To%20First
  ;[1 1 1] Movement Control
  (bind _track (Timeline|SlimeLine PlayFromStart)
    (:Update
      (Transformation|SetRelativeLocation (Variables|Components|GetSlime) (Math|Vector|Lerp(Vector) "0, 0, 0" (Variables|Default|GetfirstPoint) _track) false true))
    (:Finished
      (Utilities|FlowControl|Delay (Variables|Default|GetstopDelay))
      (Variables|Default|SetNext 1)
      (Variables|Default|SetPrevious (Variables|Default|GetfirstPoint))
      (Components|Timeline|SetPlayRate (Variables|Default|GetTimeline_0) (/ 1.0 (Variables|Default|GetpatrolSpeed)))
      (CallFunction|MovingForward))))

(event Collision|EventActorBeginOverlap
  (params (OtherActor :type Actor%20Object%20Reference))
  ;[1 1 1] Actor Overlap Handling
  ;;[1 1 1] If Slimey is Hit Damage Him
  (bind _asslimey (Utilities|Casting|CastToSlimey OtherActor)
    (:then
      (Default|UpdateHealth _asslimey 25.0))
    (:CastFailed
      ;;[1 1 1] If I am hit determine damage, then damage me
      (if (Utilities|ClassIsChildOf (Utilities|GetClass OtherActor) "/Game/Ad_Nauseum/Blueprints/General/BulletGeneral.BulletGeneral_C")
        (bind _asbullet_general (Utilities|Casting|CastToBulletGeneral OtherActor))
        (if (not (Variables|/Game/Ad_Nauseum/Blueprints/General/BulletGeneral.BulletGeneral_C|GetenemyBullet _asbullet_general))
          (CallFunction|PatrolHit (Variables|/Game/Ad_Nauseum/Blueprints/General/BulletGeneral.BulletGeneral_C|Getdamage _asbullet_general)))))))

(event EventBeginPlay
  ;[1 1 1] Startup
  (Utilities|FlowControl|Sequence
    (:then_0
      ;[1 1 1] Set Current Health to Max on Start
      (Variables|Default|SetcurrentHealth (Variables|Default|GetmaxHealth))
      (Variables|Default|SetNext -1)
      (Variables|Default|SetPrevious "0, 0, 0"))
    (:then_1
      ;[1 1 1] Set Playrate
      (Components|Timeline|SetPlayRate (Variables|Default|GetSlimeLine) (/ 1.0 (Variables|Default|GetpatrolSpeed)))
      (Variables|Default|SettestRightEnd true))))

(fn ConstructionScript
  (Transformation|SetRelativeLocation (Variables|Components|GetSlime) (Math|Vector|SelectVector (Variables|Default|GetfirstPoint) "0, 0, 0" (Variables|Default|GettestRightEnd)) false false))