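; Bottom part of the snowman boss, a Paper2D enemy that fights between two X posts, hurts Slimey on contact and drops two health pickups on death.
; It loops timeline-driven jumps toward the player with force slams, a final jump to the farther post, then a charge across.
; The charge ends on completion or when damage taken during it reaches InterruptThreshold, restarting the cycle.
; Overlapping BossFloorTrigger zeroes slam velocity.
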(event OnComponentBeginOverlap(PaperSprite)
  (params (OverlappedComponent :type Primitive%20Component%20Object%20Reference) (OtherActor :type Actor%20Object%20Reference) (OtherComp :type Primitive%20Component%20Object%20Reference) (OtherBodyIndex :type Integer) (bFromSweep :type Boolean) (SweepResult :type Hit%20Result%20Structure%20%28by%20ref%29))
  ;[1 1 1] Actor Overlap Handling
  ;;[1 1 1] If Slimey is Hit Damage Him
  (bind _asslimey (Utilities|Casting|CastToSlimey OtherActor)
    (:then
      (Default|UpdateHealth _asslimey 25.0))
    (:CastFailed
      ;;[1 1 1] If I am hit determine damage, then damage me
      (if (Utilities|ClassIsChildOf (Utilities|GetClass OtherActor) "/Game/Ad_Nauseum/Blueprints/General/BulletGeneral.BulletGeneral_C")
        (bind _asbullet_general (Utilities|Casting|CastToBulletGeneral OtherActor))
        (if (not (Variables|/Game/Ad_Nauseum/Blueprints/General/BulletGeneral.BulletGeneral_C|GetenemyBullet _asbullet_general))
          (CallFunction|PatrolHit (Variables|/Game/Ad_Nauseum/Blueprints/General/BulletGeneral.BulletGeneral_C|Getdamage _asbullet_general)))
        (else
          (Utilities|Casting|CastToBossFloorTrigger OtherActor)
          (Physics|SetPhysicsLinearVelocity (Variables|Default|GetPaperSprite) "0, 0, 0" false "None"))))))

(event Custom|FinalJump
  (bind _papersprite (Variables|Default|GetPaperSprite))
  (bind _returnvalue (Transformation|GetWorldLocation _papersprite))
  ;[1 1 1] Slightly Different Boss Jump Block
  (Utilities|FlowControl|Sequence
    (:then_0
      (Variables|Default|SetJumpStartLocation (Transformation|GetWorldLocation (Variables|Default|GetPaperSprite))))
    (:then_1
      (if (> (- (Variables|Default|GetRightPost) (.x _returnvalue)) (- (.x _returnvalue) (Variables|Default|GetLeftPost)))
        (Variables|Default|SetJumpEndLocation (Math|Vector|MakeVector (Variables|Default|GetRightPost) 0.0 (+ (Variables|Default|GetJumpHeight) (.z (Variables|Default|GetJumpStartLocation)))))
        (else
          (Variables|Default|SetJumpEndLocation (Math|Vector|MakeVector (Variables|Default|GetLeftPost) 0.0 (+ (.z (Variables|Default|GetJumpStartLocation)) (Variables|Default|GetJumpHeight)))))))
    (:then_2
      (bind _newtrack_1 (Timeline|banana PlayFromStart)
        (:Update
          (Transformation|SetActorLocation (Math|Vector|MakeVector (+ (* _newtrack_1 (- (.x (Variables|Default|GetJumpEndLocation)) (.x (Variables|Default|GetJumpStartLocation)))) (.x (Variables|Default|GetJumpStartLocation))) 0.0 (+ (.z (Variables|Default|GetJumpStartLocation)) (* _newtrack_1 (- (.z (Variables|Default|GetJumpEndLocation)) (.z (Variables|Default|GetJumpStartLocation)))))) false false))
        (:Finished
          (Physics|AddForce (Variables|Default|GetPaperSprite) (Math|Vector|MakeVector 0.0 0.0 (Variables|Default|GetSlamForce)) "None" false)
          (Utilities|FlowControl|Delay 1.0)
          (CallFunction|ChargeForward))))))

(event Custom|PatrolHit
  (params (DamageIn :type Float%20%28single-precision%29))
  (bind _returnvalue (Transformation|GetActorLocation))
  (bind _returnvalue_2 (- (.z _returnvalue) 1.8e+02))
  ;[1 1 1] Damage Me
  (bind _output_get (Variables|Default|SetcurrentHealth (- (Variables|Default|GetcurrentHealth) DamageIn)))
  ;[1 1 1] Kill me if health is <= 0
  (if (<= _output_get 0.0)
    (Game|SpawnActorfromClass "/Game/Ad_Nauseum/Blueprints/General/HealthPickup.HealthPickup_C" (Math|Transform|MakeTransform (Math|Vector|MakeVector (.x _returnvalue) (.y _returnvalue) _returnvalue_2) "0, 0, 0" "1,1,1") "Undefined" 0 0)
    (Game|SpawnActorfromClass "/Game/Ad_Nauseum/Blueprints/General/HealthPickup.HealthPickup_C" (Math|Transform|MakeTransform (Math|Vector|MakeVector (+ (.x _returnvalue) 4e+01) (.y _returnvalue) _returnvalue_2) "0, 0, 0" "1,1,1") "Undefined" 0 0)
    (Actor|DestroyActor)
    (elif (Variables|Default|GetCharging)
      (bind _output_get_2 (Variables|Default|SetInterruptDamage (+ (Variables|Default|GetInterruptDamage) DamageIn)))
      (if (>= _output_get_2 (Variables|Default|GetInterruptThreshold))
        (CallFunction|StopCharge)))))

(event Custom|BossJump
  (bind _leftpost (Variables|Default|GetLeftPost))
  ;[1 1 1] Boss Jump Block
  (Utilities|FlowControl|Sequence
    (:then_0
      (Variables|Default|SetJumpStartLocation (Transformation|GetWorldLocation (Variables|Default|GetPaperSprite))))
    (:then_1
      (bind _output_get (Variables|Default|Settemp (.x (Transformation|GetActorLocation (Game|Player|GetPlayerPawn 0)))))
      (if (> _output_get (Variables|Default|GetRightPost))
        (Variables|Default|Settemp (Variables|Default|GetRightPost))
        (elif (< _output_get _leftpost)
          (Variables|Default|Settemp _leftpost)))
      (Variables|Default|SetJumpEndLocation (Math|Vector|MakeVector (Variables|Default|Gettemp) 0.0 (+ (Variables|Default|GetJumpHeight) (.z (Variables|Default|GetJumpStartLocation))))))
    (:then_2
      (bind _newtrack_0 (Timeline|butterscotch PlayFromStart)
        (:Update
          (Transformation|SetActorLocation (Math|Vector|MakeVector (+ (* _newtrack_0 (- (.x (Variables|Default|GetJumpEndLocation)) (.x (Variables|Default|GetJumpStartLocation)))) (.x (Variables|Default|GetJumpStartLocation))) 0.0 (+ (.z (Variables|Default|GetJumpStartLocation)) (* _newtrack_0 (- (.z (Variables|Default|GetJumpEndLocation)) (.z (Variables|Default|GetJumpStartLocation)))))) false false))
        (:Finished
          (Variables|Default|SetJumpCount (- (Variables|Default|GetJumpCount) 1))
          (Physics|AddForce (Variables|Default|GetPaperSprite) (Math|Vector|MakeVector 0.0 0.0 (Variables|Default|GetSlamForce)) "None" false)
          (Utilities|FlowControl|Delay 2.0)
          (if (> (Variables|Default|GetJumpCount) 0)
            (CallFunction|BossJump)
            (else
              (CallFunction|FinalJump))))))))

(event Custom|ChargeForward
  (bind _returnvalue (Transformation|GetActorLocation))
  (bind _papersprite (Variables|Default|GetPaperSprite))
  (bind _rightpost (Variables|Default|GetRightPost))
  (bind _leftpost (Variables|Default|GetLeftPost))
  (bind _returnvalue_2 (Transformation|GetWorldLocation _papersprite))
  ;[1 1 1] Charge Forward!
  (Utilities|FlowControl|Sequence
    (:then_0
      (if (< (- (Variables|Default|GetRightPost) (.x _returnvalue_2)) (- (.x _returnvalue_2) (Variables|Default|GetLeftPost)))
        (Variables|Default|SetClosepost _rightpost)
        (Variables|Default|SetFarpost _leftpost)
        (else
          (Variables|Default|SetClosepost _leftpost)
          (Variables|Default|SetFarpost _rightpost))))
    (:then_1
      (Variables|Default|SetInterruptDamage 0.0)
      (Variables|Default|SetCharging true))
    (:then_2
      (bind _newtrack_0 (Timeline|ChargeTimeline PlayFromStart)
        (:Update
          (Transformation|SetActorLocation (Math|Vector|MakeVector (+ (* _newtrack_0 (- (Variables|Default|GetFarpost) (Variables|Default|GetClosepost))) (Variables|Default|GetClosepost)) (.y _returnvalue) (.z _returnvalue)) false false))
        (:Finished
          (CallFunction|StopCharge))))))

(event Custom|StopCharge
  (bind _returnvalue (Transformation|GetActorLocation))
  (bind _closepost (Variables|Default|GetClosepost))
  (Utilities|FlowControl|Sequence
    (:then_0
      ;[1 1 1] Charge Forward!
      (bind _newtrack_0 (Timeline|ChargeTimeline Stop)
        (:Update
          (Transformation|SetActorLocation (Math|Vector|MakeVector (+ (* _newtrack_0 (- (Variables|Default|GetFarpost) _closepost)) _closepost) (.y _returnvalue) (.z _returnvalue)) false false))
        (:Finished
          (CallFunction|StopCharge))))
    (:then_1
      (Variables|Default|SetCharging false))
    (:then_2
      (Utilities|FlowControl|Delay 3.0)
      (Variables|Default|SetJumpCount 3)
      (CallFunction|BossJump))))

(event EventBeginPlay
  ;[1 1 1] On Startup
  (Utilities|FlowControl|Sequence
    (:then_2
      (Utilities|FlowControl|Delay 1.5)
      (CallFunction|BossJump))))

(event Collision|EventActorBeginOverlap
  (params (OtherActor :type Actor%20Object%20Reference)))

(event EventTick
  (params (DeltaSeconds :type Float%20%28single-precision%29)))

(fn ConstructionScript)