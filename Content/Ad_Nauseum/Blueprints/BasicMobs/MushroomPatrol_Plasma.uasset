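; Patrolling mushroom enemy that damages Slimey on overlap and takes damage from non-enemy bullets.
; A timeline lerps the mushroom between its origin and RightEndPoint, pausing before each reversal; nothing here makes the first MovingForward call.
; At zero health it always drops a plasma pickup despite the random switch, as the health pickup branch is unwired.
; The construction script uses TestRightEnd to preview either patrol endpoint.
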(event Custom|Moving%20Forward
  ;[1 1 1] Movement Control
  (bind (_direction _driver) (Timeline|PatrolTimeline PlayFromStart)
    (:Update
      (Transformation|SetRelativeLocation (Variables|Default|GetMushroomPatroler) (Math|Vector|Lerp(Vector) "0, 0, 0" (Variables|Default|GetrightEndPoint) _driver) false false))
    (:Finished
      (Utilities|FlowControl|Delay (Variables|Default|GetstopDelay))
      (switch Utilities|FlowControl|Switch|SwitchonETimelineDirection _direction
        (:Forward
          (CallFunction|MovingBackward))
        (:Backward
          (CallFunction|MovingForward))))))

(event Custom|PatrolHit
  (params (DamageIn :type Float%20%28single-precision%29))
  ;[1 1 1] Damage Me
  (bind _output_get (Variables|Default|SetcurrentHealth (- (Variables|Default|GetcurrentHealth) DamageIn)))
  ;[1 1 1] Kill me if health is <= 0
  (if (<= _output_get 0.0)
    ;[1 1 1] Spawn any loot upon death
    (switch int (Math|Random|RandomIntegerinRange 0 2)
      (:0
        _)
      (:1
        _)
      (:2
        _))
    (Game|SpawnActorfromClass "/Game/Ad_Nauseum/Blueprints/General/PlasmaPickup.PlasmaPickup_C" (Transformation|GetWorldTransform (Variables|Default|GetMushroomPatroler)) "Undefined" 0 0)
    (Actor|DestroyActor)))

(event Custom|Moving%20Backward
  ;[1 1 1] Movement Control
  (bind (_direction _driver) (Timeline|PatrolTimeline ReverseFromEnd)
    (:Update
      (Transformation|SetRelativeLocation (Variables|Default|GetMushroomPatroler) (Math|Vector|Lerp(Vector) "0, 0, 0" (Variables|Default|GetrightEndPoint) _driver) false false))
    (:Finished
      (Utilities|FlowControl|Delay (Variables|Default|GetstopDelay))
      (switch Utilities|FlowControl|Switch|SwitchonETimelineDirection _direction
        (:Forward
          (CallFunction|MovingBackward))
        (:Backward
          (CallFunction|MovingForward))))))

(event Collision|EventActorBeginOverlap
  (params (OtherActor :type Actor%20Object%20Reference))
  ;[1 1 1] Actor Overlap Handling
  ;;[1 1 1] If Slimey is Hit Damage Him
  (bind _asslimey (Utilities|Casting|CastToSlimey OtherActor)
    (:then
      (Default|UpdateHealth _asslimey 25.0))
    (:CastFailed
      ;;[1 1 1] If I am hit determine damage, then damage me
      (if (Utilities|ClassIsChildOf (Utilities|GetClass OtherActor) "/Game/Ad_Nauseum/Blueprints/General/BulletGeneral.BulletGeneral_C")
        (bind _asbullet_general (Utilities|Casting|CastToBulletGeneral OtherActor))
        (if (not (Variables|/Game/Ad_Nauseum/Blueprints/General/BulletGeneral.BulletGeneral_C|GetenemyBullet _asbullet_general))
          (CallFunction|PatrolHit (Variables|/Game/Ad_Nauseum/Blueprints/General/BulletGeneral.BulletGeneral_C|Getdamage _asbullet_general)))))))

(event EventBeginPlay
  ;[1 1 1] Startup
  (Utilities|FlowControl|Sequence
    (:then_0
      ;[1 1 1] Set Current Health to Max on Start
      (Variables|Default|SetcurrentHealth (Variables|Default|GetmaxHealth)))
    (:then_1
      ;[1 1 1] Set Playrate
      (Components|Timeline|SetPlayRate (Variables|Default|GetPatrolTimeline) (/ 1.0 (Variables|Default|GetpatrolSpeed)))
      (Variables|Default|SettestRightEnd true))))

(fn ConstructionScript
  (Transformation|SetRelativeLocation (Variables|Default|GetMushroomPatroler) (Math|Vector|SelectVector (Variables|Default|GetrightEndPoint) "0, 0, 0" (Variables|Default|GettestRightEnd)) false false))