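; Wisp is a shooting patrol enemy that damages Slimey on overlap and loses health to non-enemy BulletGeneral hits.
; A timeline lerps it between its origin and RightEndPoint, pausing at each end to reverse and rotate ShootPoint.
; A self-repeating delayed event fires WispFire from ShootPoint.
; On death it has a one-in-three HealthPickup drop, and the construction script uses TestRightEnd to preview either patrol end.
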(event Custom|Moving%20Forward
  ;[1 1 1] Movement Control
  (bind (_direction _driver) (Timeline|ShooterTimeline Play)
    (:Update
      (Transformation|SetRelativeLocation (Variables|Default|GetWisp) (Math|Vector|Lerp(Vector) "0, 0, 0" (Variables|Default|GetrightEndPoint) _driver) false false))
    (:Finished
      (Utilities|FlowControl|Delay (Variables|Default|GetstopDelay))
      (switch Utilities|FlowControl|Switch|SwitchonETimelineDirection _direction
        (:Forward
          (CallFunction|MovingBackward)
          (Transformation|SetRelativeRotation (Variables|Default|GetShootPoint) "0,180.000000, 0" false false))
        (:Backward
          (CallFunction|MovingForward)
          (Transformation|SetRelativeRotation (Variables|Default|GetShootPoint) "0,0.000000, 0" false false))))))

(event Custom|PatrolHit
  (params (DamageIn :type Float%20%28single-precision%29))
  ;[1 1 1] Damage Me
  (bind _output_get (Variables|Default|SetcurrentHealth (- (Variables|Default|GetcurrentHealth) DamageIn)))
  ;[1 1 1] Kill me if health is <= 0
  (if (<= _output_get 0.0)
    ;[1 1 1] Drop any Loot upon Death
    (switch int (Math|Random|RandomIntegerinRange 0 2)
      (:0
        _)
      (:1
        (Game|SpawnActorfromClass "/Game/Ad_Nauseum/Blueprints/General/HealthPickup.HealthPickup_C" (Transformation|GetWorldTransform (Variables|Default|GetWisp)) "Undefined" 0 0))
      (:2
        _))
    (Actor|DestroyActor)))

(event Custom|Moving%20Backward
  ;[1 1 1] Movement Control
  (bind (_direction _driver) (Timeline|ShooterTimeline ReverseFromEnd)
    (:Update
      (Transformation|SetRelativeLocation (Variables|Default|GetWisp) (Math|Vector|Lerp(Vector) "0, 0, 0" (Variables|Default|GetrightEndPoint) _driver) false false))
    (:Finished
      (Utilities|FlowControl|Delay (Variables|Default|GetstopDelay))
      (switch Utilities|FlowControl|Switch|SwitchonETimelineDirection _direction
        (:Forward
          (CallFunction|MovingBackward)
          (Transformation|SetRelativeRotation (Variables|Default|GetShootPoint) "0,180.000000, 0" false false))
        (:Backward
          (CallFunction|MovingForward)
          (Transformation|SetRelativeRotation (Variables|Default|GetShootPoint) "0,0.000000, 0" false false))))))

(event Custom|Shoot%20Bullet
  ;[1 1 1] Shoot Bullet every X seconds based on shotDelay
  (Game|SpawnActorfromClass "/Game/Ad_Nauseum/Blueprints/Weapons/WispFire.WispFire_C" (Transformation|GetWorldTransform (Variables|Default|GetShootPoint)) "AlwaysSpawn" 0 0)
  (Utilities|FlowControl|Delay (Variables|Default|GetshotDelay))
  (CallFunction|ShootBullet))

(event Collision|EventActorBeginOverlap
  (params (OtherActor :type Actor%20Object%20Reference))
  ;[1 1 1] Actor Overlap Handling
  ;;[1 1 1] If Slimey is Hit Damage Him
  (bind _asslimey (Utilities|Casting|CastToSlimey OtherActor)
    (:then
      (Default|UpdateHealth _asslimey 25.0))
    (:CastFailed
      ;;[1 1 1] If I am hit determine damage, then damage me
      (if (Utilities|ClassIsChildOf (Utilities|GetClass OtherActor) "/Game/Ad_Nauseum/Blueprints/General/BulletGeneral.BulletGeneral_C")
        (bind _asbullet_general (Utilities|Casting|CastToBulletGeneral OtherActor))
        (if (not (Variables|/Game/Ad_Nauseum/Blueprints/General/BulletGeneral.BulletGeneral_C|GetenemyBullet _asbullet_general))
          (CallFunction|PatrolHit (Variables|/Game/Ad_Nauseum/Blueprints/General/BulletGeneral.BulletGeneral_C|Getdamage _asbullet_general)))))))

(event EventBeginPlay
  ;[1 1 1] Startup
  (Utilities|FlowControl|Sequence
    (:then_0
      ;[1 1 1] Set Current Health to Max on Start
      (Variables|Default|SetcurrentHealth (Variables|Default|GetmaxHealth)))
    (:then_1
      ;[1 1 1] Set Playrate
      (Components|Timeline|SetPlayRate (Variables|Default|GetShooterTimeline) (/ 1.0 (Variables|Default|GetpatrolSpeed)))
      (Variables|Default|SettestRightEnd true))
    (:then_2
      (CallFunction|ShootBullet))))

(fn ConstructionScript
  (Transformation|SetRelativeLocation (Variables|Default|GetWisp) (Math|Vector|SelectVector (Variables|Default|GetrightEndPoint) "0, 0, 0" (Variables|Default|GettestRightEnd)) false false))