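; Scorpion boss Blueprint that spawns tail segments, stinger and claw as separate actors and shows a HUD health bar.
; ScorpionAttack randomly picks timeline-driven attacks: a tail strike firing a missile at Slimey, or a claw slam dropping eggs.
; Tick stages vulnerability: repeated stinger kills remove the tail and expose the claw, whose death exposes the body.
; Each stage damages shared health; death spawns the End_Goal to Level_7.
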(event Custom|ScorpionHit
  (params (DamageIn :type Float%20%28single-precision%29))
  ;[1 1 1] Damage Me
  (bind _output_get (Variables|Health|SetcurrentHealth (- (Variables|Health|GetcurrentHealth) DamageIn)))
  ;[1 1 1] Update Health Bar
  (Progress|SetPercent (Variables|/Game/Ad_Nauseum/Blueprints/General/BossHUD.BossHUD_C|GetScorpionHealth (Variables|Health|GetbossHealth)) (/ _output_get (Variables|Health|GetmaxHealth)))
  ;[1 1 1] Kill me if health is <= 0
  (if (<= _output_get 0.0)
    (Utilities|FlowControl|Sequence
      (:then_0
        ;[1 1 1] Scorpion Dead Remove His Healthbar
        (Widget|RemovefromParent (Variables|Health|GetbossHealth)))
      (:then_1
        (bind _returnvalue (Game|SpawnActorfromClass "/Game/Ad_Nauseum/Blueprints/General/End_Goal.End_Goal_C" (Math|Transform|MakeTransform "5816.000000, 0,-931.000000" "0, 0, 0" "1,1,1") "Undefined" 0 0))
        (Variables|/Game/Ad_Nauseum/Blueprints/General/End_Goal.End_Goal_C|SetlevelName _returnvalue "Level_7")
        (Actor|DestroyActor)))))

(event Custom|Stinger%20Done
  (bind _arrow (Variables|Default|GetArrow))
  (bind _returnvalue (Transformation|GetWorldTransform _arrow))
  ;[1 1 1] Tail Sequence: To Add Projectile Fire
  (bind (_direction _stinger_move) (Timeline|Stinger_Timeline ReverseFromEnd)
    (:Update
      (CallFunction|TailMove _stinger_move))
    (:Finished
      (switch Utilities|FlowControl|Switch|SwitchonETimelineDirection _direction
        (:Forward
          (bind _asslimey (Utilities|Casting|CastToSlimey (Game|Player|GetPlayerPawn 0)))
          (Game|SpawnActorfromClass "/Game/Ad_Nauseum/Blueprints/Scorpion/Stinger_Missile.Stinger_Missile_C" (Math|Transform|MakeTransform (.location _returnvalue) (Math|Rotator|FindLookatRotation (.location _returnvalue) (Transformation|GetWorldLocation (Variables|/Script/Engine.Character|GetCapsuleComponent _asslimey)))) "AlwaysSpawn" 0 0)
          (Utilities|FlowControl|Delay 1.0)
          (CallFunction|StingerDone))))))

(event Custom|Scorpion%20Attack
  ;[1 1 1] Attack Determiner
  (if (not (Variables|Booleans|GetstingerDead))
    (switch int (Math|Random|RandomIntegerinRange 0 1)
      (:0
        (CallFunction|StingerHit))
      (:1
        (CallFunction|ClawSlam)))
    (Utilities|FlowControl|Delay 5.0 :!label _label)
    (CallFunction|ScorpionAttack)
    (elif (not (Variables|Booleans|GetclawDead))
      (switch int (Math|Random|RandomIntegerinRange 0 1)
        (:0
          (CallFunction|ClawSlam)
          (goto _label)))
      (else
        (CallFunction|BodySlam)))))

(event Custom|Stinger%20Hit
  (bind _arrow (Variables|Default|GetArrow))
  (bind _returnvalue (Transformation|GetWorldTransform _arrow))
  ;[1 1 1] Tail Sequence: To Add Projectile Fire
  (bind (_direction _stinger_move) (Timeline|Stinger_Timeline PlayFromStart)
    (:Update
      (CallFunction|TailMove _stinger_move))
    (:Finished
      (switch Utilities|FlowControl|Switch|SwitchonETimelineDirection _direction
        (:Forward
          (bind _asslimey (Utilities|Casting|CastToSlimey (Game|Player|GetPlayerPawn 0)))
          (Game|SpawnActorfromClass "/Game/Ad_Nauseum/Blueprints/Scorpion/Stinger_Missile.Stinger_Missile_C" (Math|Transform|MakeTransform (.location _returnvalue) (Math|Rotator|FindLookatRotation (.location _returnvalue) (Transformation|GetWorldLocation (Variables|/Script/Engine.Character|GetCapsuleComponent _asslimey)))) "AlwaysSpawn" 0 0)
          (Utilities|FlowControl|Delay 1.0)
          (CallFunction|StingerDone))))))

(event Custom|Claw%20Slam
  (bind _bodylocation (Variables|Locations|GetbodyLocation))
  (bind _clawlocation (Variables|Locations|GetclawLocation))
  (bind _returnvalue (+ _bodylocation _clawlocation))
  ;[1 1 1] Claw Slam
  (bind (_direction _slam_track) (Timeline|Slam_Timeline PlayFromStart)
    (:Update
      (Transformation|SetActorRelativeLocation (Variables|Tail|Getclaw) (Math|Vector|Lerp(Vector) _returnvalue (+ _returnvalue "0.000000, 0,25.000000") _slam_track)))
    (:Finished
      (switch Utilities|FlowControl|Switch|SwitchonETimelineDirection _direction
        (:Forward
          (CallFunction|SlamReverse))
        (:Backward
          (Game|SpawnActorfromClass "/Game/Ad_Nauseum/Blueprints/Scorpion/Falling_Eggs.Falling_Eggs_C" (Math|Transform|MakeTransform (+ (Variables|Locations|GetbodyLocation) (Variables|Default|GeteggSpawn1)) "0, 0, 0" "1,1,1") "Undefined" 0 0)
          (Utilities|FlowControl|Delay 2.0))))))

(event Custom|Claw%20Swipe
  (bind _bodylocation (Variables|Locations|GetbodyLocation))
  (bind _clawlocation (Variables|Locations|GetclawLocation))
  (bind _returnvalue (+ _bodylocation _clawlocation))
  ;[1 1 1] Claw Swipe
  (bind (_direction _swipe_curve) (Timeline|Claw%20Swipe%20Timeline PlayFromStart)
    (:Update
      (Transformation|SetActorRelativeLocation (Variables|Tail|Getclaw) (Math|Vector|Lerp(Vector) _returnvalue (+ _returnvalue "-25.000000, 0, 0") _swipe_curve)))
    (:Finished
      (switch Utilities|FlowControl|Switch|SwitchonETimelineDirection _direction
        (:Forward
          (CallFunction|ReverseClaw))))))

(event Custom|Reverse%20Claw
  (bind _bodylocation (Variables|Locations|GetbodyLocation))
  (bind _clawlocation (Variables|Locations|GetclawLocation))
  (bind _returnvalue (+ _bodylocation _clawlocation))
  ;[1 1 1] Claw Swipe
  (bind (_direction _swipe_curve) (Timeline|Claw%20Swipe%20Timeline ReverseFromEnd)
    (:Update
      (Transformation|SetActorRelativeLocation (Variables|Tail|Getclaw) (Math|Vector|Lerp(Vector) _returnvalue (+ _returnvalue "-25.000000, 0, 0") _swipe_curve)))
    (:Finished
      (switch Utilities|FlowControl|Switch|SwitchonETimelineDirection _direction
        (:Forward
          (CallFunction|ReverseClaw))))))

(event Custom|Body%20Slam
  ;[1 1 1] Spawns Eggs
  (Game|SpawnActorfromClass "/Game/Ad_Nauseum/Blueprints/Scorpion/Falling_Eggs.Falling_Eggs_C" (Math|Transform|MakeTransform (+ (Variables|Locations|GetbodyLocation) (Variables|Default|GeteggSpawn1)) "0, 0, 0" "1,1,1") "Undefined" 0 0)
  (Utilities|FlowControl|Delay 3.0))

(event Custom|Slam%20Reverse
  (bind _bodylocation (Variables|Locations|GetbodyLocation))
  (bind _clawlocation (Variables|Locations|GetclawLocation))
  (bind _returnvalue (+ _bodylocation _clawlocation))
  ;[1 1 1] Claw Slam
  (bind (_direction _slam_track) (Timeline|Slam_Timeline ReverseFromEnd)
    (:Update
      (Transformation|SetActorRelativeLocation (Variables|Tail|Getclaw) (Math|Vector|Lerp(Vector) _returnvalue (+ _returnvalue "0.000000, 0,25.000000") _slam_track)))
    (:Finished
      (switch Utilities|FlowControl|Switch|SwitchonETimelineDirection _direction
        (:Forward
          (CallFunction|SlamReverse))
        (:Backward
          (Game|SpawnActorfromClass "/Game/Ad_Nauseum/Blueprints/Scorpion/Falling_Eggs.Falling_Eggs_C" (Math|Transform|MakeTransform (+ (Variables|Locations|GetbodyLocation) (Variables|Default|GeteggSpawn1)) "0, 0, 0" "1,1,1") "Undefined" 0 0)
          (Utilities|FlowControl|Delay 2.0))))))

(event EventBeginPlay
  (bind _maxhealth (Variables|Health|GetmaxHealth))
  ;[1 1 1] Init
  (Utilities|FlowControl|Sequence
    (:then_0
      ;;[1 1 1] Add Scorpion Healthbar to Viewport
      (bind _returnvalue (UserInterface|CreateWidget "/Game/Ad_Nauseum/Blueprints/General/BossHUD.BossHUD_C"))
      (bind _output_get (Variables|Health|SetbossHealth _returnvalue))
      (UserInterface|Viewport|AddtoViewport _output_get 0))
    (:then_1
      ;;[1 1 1] initialize Health and Health bar
      (bind _output_get_2 (Variables|Health|SetcurrentHealth _maxhealth))
      (Progress|SetPercent (Variables|/Game/Ad_Nauseum/Blueprints/General/BossHUD.BossHUD_C|GetScorpionHealth (Variables|Health|GetbossHealth)) (/ _output_get_2 _maxhealth)))
    (:then_2
      ;;[1 1 1] Set the location of the Scorpions Body
      (Variables|Locations|SetbodyLocation (Transformation|GetWorldLocation (Variables|Components|GetRoot))))
    (:then_3
      ;;[1 1 1] Spawn Tail Segments
      (bind _returnvalue_2 (Game|SpawnActorfromClass "/Game/Ad_Nauseum/Blueprints/Scorpion/Scorpion_Tail_Segment.Scorpion_Tail_Segment_C" (Math|Transform|MakeTransform (+ (Variables|Locations|GetbodyLocation) (Variables|Locations|GettailSeg1Location)) "0, 0, 0" "1,1,1") "Undefined" 0 0))
      (Variables|Tail|SettailSeg1 _returnvalue_2)
      (bind _returnvalue_3 (Game|SpawnActorfromClass "/Game/Ad_Nauseum/Blueprints/Scorpion/Scorpion_Tail_Segment.Scorpion_Tail_Segment_C" (Math|Transform|MakeTransform (+ (Variables|Locations|GetbodyLocation) (Variables|Locations|GettailSeg2Location)) "0, 0, 0" "1,1,1") "Undefined" 0 0))
      (Variables|Tail|SettailSeg2 _returnvalue_3)
      (bind _returnvalue_4 (Game|SpawnActorfromClass "/Game/Ad_Nauseum/Blueprints/Scorpion/Scorpion_Tail_Segment.Scorpion_Tail_Segment_C" (Math|Transform|MakeTransform (+ (Variables|Locations|GetbodyLocation) (Variables|Locations|GettailSeg3Location)) "0, 0, 0" "1,1,1") "Undefined" 0 0))
      (Variables|Tail|SettailSeg3 _returnvalue_4)
      (bind _returnvalue_5 (Game|SpawnActorfromClass "/Game/Ad_Nauseum/Blueprints/Scorpion/Scorpion_Tail_Segment.Scorpion_Tail_Segment_C" (Math|Transform|MakeTransform (+ (Variables|Locations|GetbodyLocation) (Variables|Locations|GettailSeg4Location)) "0, 0, 0" "1,1,1") "Undefined" 0 0))
      (Variables|Tail|SettailSeg4 _returnvalue_5))
    (:then_4
      ;;[1 1 1] Spawn the Stinger
      (bind _returnvalue_6 (Game|SpawnActorfromClass "/Game/Ad_Nauseum/Blueprints/Scorpion/Scorpion_Stinger.Scorpion_Stinger_C" (Math|Transform|MakeTransform (+ (Variables|Locations|GetbodyLocation) (Variables|Locations|GetstingerLocation)) "0, 0, 0" "1,1,1") "Undefined" 0 0))
      (Variables|Tail|Setstinger _returnvalue_6))
    (:then_5
      ;;[1 1 1] Spawn Claw
      (bind _returnvalue_7 (Game|SpawnActorfromClass "/Game/Ad_Nauseum/Blueprints/Scorpion/Scorpion_Claw.Scorpion_Claw_C" (Math|Transform|MakeTransform (+ (Variables|Locations|GetbodyLocation) (Variables|Locations|GetclawLocation)) "0, 0, 0" "1,1,1") "Undefined" 0 0))
      (Variables|Tail|Setclaw _returnvalue_7))
    (:then_6
      (Utilities|FlowControl|Delay 1.0)
      (CallFunction|ScorpionAttack))))

(event Collision|EventActorBeginOverlap
  (params (OtherActor :type Actor%20Object%20Reference))
  ;[1 1 1] Actor Overlap Handling
  ;;[1 1 1] If Slimey is Hit Damage Him
  (bind _asslimey (Utilities|Casting|CastToSlimey OtherActor)
    (:then
      (Default|UpdateHealth _asslimey 25.0))
    (:CastFailed
      ;;[1 1 1] If I am hit determine damage, then damage me
      (if (Utilities|ClassIsChildOf (Utilities|GetClass OtherActor) "/Game/Ad_Nauseum/Blueprints/General/BulletGeneral.BulletGeneral_C")
        (bind _asbullet_general (Utilities|Casting|CastToBulletGeneral OtherActor))
        (if (not (Variables|/Game/Ad_Nauseum/Blueprints/General/BulletGeneral.BulletGeneral_C|GetenemyBullet _asbullet_general))
          (if (Variables|Booleans|GetbodyDamageable)
            (CallFunction|ScorpionHit (Variables|/Game/Ad_Nauseum/Blueprints/General/BulletGeneral.BulletGeneral_C|Getdamage _asbullet_general))))))))

(event EventTick
  (params (DeltaSeconds :type Float%20%28single-precision%29))
  (bind _killdelay (Variables|Default|GetkillDelay))
  (bind _claw (Variables|Tail|Getclaw))
  (bind _stinger (Variables|Tail|Getstinger))
  ;[1 1 1] On Tick
  (if (Variables|Booleans|GetstingerDead)
    (if (Variables|Booleans|GetsegmentsDead)
      ;;[1 1 1] Check Claw Status
      (if (not (Variables|Booleans|GetclawDead))
        (if (Variables|/Game/Ad_Nauseum/Blueprints/Scorpion/Scorpion_Claw.Scorpion_Claw_C|Getdead _claw)
          (Actor|DestroyActor _claw)
          (Variables|Booleans|SetclawDead true)
          (Variables|Booleans|SetbodyDamageable true)
          (CallFunction|ScorpionHit 25.0))))
    (else
      ;;[1 1 1] Stinger Hit Handler
      (if (Variables|/Game/Ad_Nauseum/Blueprints/Scorpion/Scorpion_Stinger.Scorpion_Stinger_C|Getdead _stinger)
        (bind _output_get (Variables|Default|SetstingerHits (+ (Variables|Default|GetstingerHits) 1)))
        (if (== _output_get (Variables|Default|GetstingerMaxHits))
          (Variables|Booleans|SetstingerDead true)
          (CallFunction|ScorpionHit 25.0)
          (Actor|DestroyActor _stinger)
          (Utilities|FlowControl|Delay _killdelay)
          (Actor|DestroyActor (Variables|Tail|GettailSeg4))
          (Utilities|FlowControl|Delay _killdelay)
          (Actor|DestroyActor (Variables|Tail|GettailSeg3))
          (Utilities|FlowControl|Delay _killdelay)
          (Actor|DestroyActor (Variables|Tail|GettailSeg2))
          (Utilities|FlowControl|Delay _killdelay)
          (Actor|DestroyActor (Variables|Tail|GettailSeg1))
          (bind _output_get_2 (Variables|Booleans|SetsegmentsDead true))
          (bind _output_get_3 (Variables|Booleans|SetstingerDead _output_get_2))
          (Variables|/Game/Ad_Nauseum/Blueprints/Scorpion/Scorpion_Claw.Scorpion_Claw_C|Setdamageable (Variables|Tail|Getclaw) _output_get_3)
          (else
            (Variables|/Game/Ad_Nauseum/Blueprints/Scorpion/Scorpion_Stinger.Scorpion_Stinger_C|Setdead _stinger false)
            (Variables|/Game/Ad_Nauseum/Blueprints/Scorpion/Scorpion_Stinger.Scorpion_Stinger_C|SetcurrentHealth _stinger (Variables|/Game/Ad_Nauseum/Blueprints/Scorpion/Scorpion_Stinger.Scorpion_Stinger_C|GetmaxHealth _stinger))
            (CallFunction|ScorpionHit 25.0)))))))

(fn ConstructionScript)

(fn TailMove
  (params (Alpha :type Float%20%28single-precision%29))
  (Transformation|SetActorRelativeLocation (Variables|Tail|GettailSeg2) (Math|Vector|Lerp(Vector) (+ (Variables|Locations|GetbodyLocation) (Variables|Locations|GettailSeg2Location)) (+ (Variables|Locations|GetbodyLocation) (Variables|Default|GetattackSeg2)) Alpha))
  (Transformation|SetActorRelativeLocation (Variables|Tail|GettailSeg3) (Math|Vector|Lerp(Vector) (+ (Variables|Locations|GetbodyLocation) (Variables|Locations|GettailSeg3Location)) (+ (Variables|Locations|GetbodyLocation) (Variables|Default|GetattackSeg3)) Alpha))
  (Transformation|SetActorRelativeLocation (Variables|Tail|GettailSeg4) (Math|Vector|Lerp(Vector) (+ (Variables|Locations|GetbodyLocation) (Variables|Locations|GettailSeg4Location)) (+ (Variables|Locations|GetbodyLocation) (Variables|Default|GetattackSeg4)) Alpha))
  (Transformation|SetActorRelativeLocation (Variables|Tail|Getstinger) (Math|Vector|Lerp(Vector) (+ (Variables|Locations|GetbodyLocation) (Variables|Locations|GetstingerLocation)) (+ (Variables|Locations|GetbodyLocation) (Variables|Default|GetattackStinger)) Alpha)))