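; Scorpion egg projectile that falls straight down, damages Slimey on overlap and hatches Baby_Scorpions on the ground.
; A GroundCheck overlap destroys it shortly after touching Slimey, while touching the tile map makes it damageable and starts spawning.
; SpawnBabies calls itself after delays, producing babies at BabyPoint indefinitely until the egg is destroyed.
; Once damageable, non-enemy BulletGeneral hits reduce its health and destroy it at zero.
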(event OnComponentBeginOverlap(GroundCheck)
  (params (OverlappedComponent :type Primitive%20Component%20Object%20Reference) (OtherActor :type Actor%20Object%20Reference) (OtherComp :type Primitive%20Component%20Object%20Reference) (OtherBodyIndex :type Integer) (bFromSweep :type Boolean) (SweepResult :type Hit%20Result%20Structure%20%28by%20ref%29))
  (Utilities|Casting|CastToPaperTileMapActor OtherActor
    (:then
      (Variables|Default|Setdamageable true)
      (CallFunction|SpawnBabies))
    (:CastFailed
      (Utilities|Casting|CastToSlimey OtherActor)
      (Utilities|FlowControl|Delay 0.2)
      (Actor|DestroyActor))))

(event Custom|PatrolHit
  (params (DamageIn :type Float%20%28single-precision%29))
  ;[1 1 1] Damage Me
  (bind _output_get (Variables|Default|SetcurrentHealth (- (Variables|Default|GetcurrentHealth) DamageIn)))
  ;[1 1 1] Kill me if health is <= 0
  (if (<= _output_get 0.0)
    (Actor|DestroyActor)))

(event Custom|Spawn%20Babies
  (Game|SpawnActorfromClass "/Game/Ad_Nauseum/Blueprints/Scorpion/Baby_Scorpion.Baby_Scorpion_C" (Transformation|GetWorldTransform (Variables|Default|Getbaby_point)) "Undefined" 0 0)
  (Utilities|FlowControl|Delay 0.5)
  (Game|SpawnActorfromClass "/Game/Ad_Nauseum/Blueprints/Scorpion/Baby_Scorpion.Baby_Scorpion_C" (Transformation|GetWorldTransform (Variables|Default|Getbaby_point)) "Undefined" 0 0)
  (Utilities|FlowControl|Delay 1.0)
  (CallFunction|SpawnBabies))

(event EventBeginPlay
  (Variables|/Script/Engine.MovementComponent|SetVelocity (Variables|Default|GetProjectileMovement) "0,0.000000,-400.000000")
  (Variables|Default|SetcurrentHealth (Variables|Default|GetmaxHealth)))

(event Collision|EventActorBeginOverlap
  (params (OtherActor :type Actor%20Object%20Reference))
  ;[1 1 1] Actor Overlap Handling
  ;;[1 1 1] If Slimey is Hit Damage Him
  (bind _asslimey (Utilities|Casting|CastToSlimey OtherActor)
    (:then
      (Default|UpdateHealth _asslimey 25.0))
    (:CastFailed
      ;;[1 1 1] If I am hit determine damage, then damage me
      (if (Utilities|ClassIsChildOf (Utilities|GetClass OtherActor) "/Game/Ad_Nauseum/Blueprints/General/BulletGeneral.BulletGeneral_C")
        (bind _asbullet_general (Utilities|Casting|CastToBulletGeneral OtherActor))
        (if (not (Variables|/Game/Ad_Nauseum/Blueprints/General/BulletGeneral.BulletGeneral_C|GetenemyBullet _asbullet_general))
          (if (Variables|Default|Getdamageable)
            (CallFunction|PatrolHit (Variables|/Game/Ad_Nauseum/Blueprints/General/BulletGeneral.BulletGeneral_C|Getdamage _asbullet_general))))))))

(fn ConstructionScript)