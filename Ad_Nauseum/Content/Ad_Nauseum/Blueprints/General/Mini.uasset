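; Mini is an actor Blueprint, apparently a miniature player form that swaps back into a Slimey.
; Pressing M unpossesses the player controller, destroys this actor, spawns a Slimey at its transform and has the controller possess the new one.
; BeginPlay, overlap and Tick events are unused, and the construction script only calls its parent.
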(event EventBeginPlay
  (|CallParentFunction))

(event Collision|EventActorBeginOverlap
  (params (OtherActor :type Actor%20Object%20Reference))
  (|CallParentFunction 0))

(event EventTick
  (params (DeltaSeconds :type Float%20%28single-precision%29))
  (|CallParentFunction 0.0))

(event Input|KeyboardEvents|M
  (params (Key :type Key%20Structure :default "AnyKey"))
  (:Pressed
    (Pawn|UnPossess (Game|GetPlayerController 0))
    (Actor|DestroyActor)
    (bind _returnvalue (Game|SpawnActorfromClass "/Game/Ad_Nauseum/Blueprints/General/Slimey.Slimey_C" (Transformation|GetActorTransform) "Undefined" 0 0))
    (Pawn|Possess (Game|GetPlayerController 0) _returnvalue)))

(fn ConstructionScript
  (|CallParentFunction))