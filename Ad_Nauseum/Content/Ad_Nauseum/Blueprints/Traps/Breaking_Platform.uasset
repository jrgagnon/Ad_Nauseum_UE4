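; Breaking platform trap that falls shortly after the Slimey character touches it.
; Overlap with either of two trigger boxes waits a second, sets ProjectileMovement to a constant downward velocity, then destroys the FallingBlock component after a further delay.
; A GroundCheck overlap with a Paper2D tile map actor also destroys FallingBlock almost immediately, removing it when it reaches the level geometry.
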(event OnComponentBeginOverlap(GroundCheck)
  (params (OverlappedComponent :type Primitive%20Component%20Object%20Reference) (OtherActor :type Actor%20Object%20Reference) (OtherComp :type Primitive%20Component%20Object%20Reference) (OtherBodyIndex :type Integer) (bFromSweep :type Boolean) (SweepResult :type Hit%20Result%20Structure%20%28by%20ref%29))
  (Utilities|Casting|CastToPaperTileMapActor OtherActor)
  (Utilities|FlowControl|Delay 0.2)
  (Components|DestroyComponent (Variables|Default|GetFalling_Block)))

(event OnComponentBeginOverlap(Box)
  (params (OverlappedComponent :type Primitive%20Component%20Object%20Reference) (OtherActor :type Actor%20Object%20Reference) (OtherComp :type Primitive%20Component%20Object%20Reference) (OtherBodyIndex :type Integer) (bFromSweep :type Boolean) (SweepResult :type Hit%20Result%20Structure%20%28by%20ref%29))
  (Utilities|Casting|CastToSlimey OtherActor)
  (Utilities|FlowControl|Delay 1.0)
  (Variables|/Script/Engine.MovementComponent|SetVelocity (Variables|Default|GetProjectileMovement) "0,0.000000,-400.000000")
  (Utilities|FlowControl|Delay 5.0)
  (Components|DestroyComponent (Variables|Default|GetFalling_Block)))

(event OnComponentBeginOverlap(Box1)
  (params (OverlappedComponent :type Primitive%20Component%20Object%20Reference) (OtherActor :type Actor%20Object%20Reference) (OtherComp :type Primitive%20Component%20Object%20Reference) (OtherBodyIndex :type Integer) (bFromSweep :type Boolean) (SweepResult :type Hit%20Result%20Structure%20%28by%20ref%29))
  (Utilities|Casting|CastToSlimey OtherActor)
  (Utilities|FlowControl|Delay 1.0)
  (Variables|/Script/Engine.MovementComponent|SetVelocity (Variables|Default|GetProjectileMovement) "0,0.000000,-400.000000")
  (Utilities|FlowControl|Delay 5.0)
  (Components|DestroyComponent (Variables|Default|GetFalling_Block)))

(event EventBeginPlay)

(event Collision|EventActorBeginOverlap
  (params (OtherActor :type Actor%20Object%20Reference)))

(event EventTick
  (params (DeltaSeconds :type Float%20%28single-precision%29)))

(fn ConstructionScript)