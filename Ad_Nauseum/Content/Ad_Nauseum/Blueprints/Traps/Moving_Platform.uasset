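; Moving platform trap that shuttles a platform component between its relative origin and a configurable right end point.
; A timeline lerps the relative location, with play rate set from the inverse of PatrolSpeed, then waits StopDelay and reverses through the MovingForward and MovingBackward events.
; BeginPlay does not call MovingForward, so nothing here starts the patrol.
; The construction script uses TestRightEnd to preview either end position.
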(event Custom|Moving%20Forward
  ;[1 1 1] Movement Control
  (bind (_direction _driver) (Timeline|PatrolTimeline PlayFromStart)
    (:Update
      (Transformation|SetRelativeLocation (Variables|Default|GetMovingPlatform) (Math|Vector|Lerp(Vector) "0, 0, 0" (Variables|Default|GetrightEndPoint) _driver) false false))
    (:Finished
      (Utilities|FlowControl|Delay (Variables|Default|GetstopDelay))
      (switch Utilities|FlowControl|Switch|SwitchonETimelineDirection _direction
        (:Forward
          (CallFunction|MovingBackward))
        (:Backward
          (CallFunction|MovingForward))))))

(event Custom|Moving%20Backward
  ;[1 1 1] Movement Control
  (bind (_direction _driver) (Timeline|PatrolTimeline ReverseFromEnd)
    (:Update
      (Transformation|SetRelativeLocation (Variables|Default|GetMovingPlatform) (Math|Vector|Lerp(Vector) "0, 0, 0" (Variables|Default|GetrightEndPoint) _driver) false false))
    (:Finished
      (Utilities|FlowControl|Delay (Variables|Default|GetstopDelay))
      (switch Utilities|FlowControl|Switch|SwitchonETimelineDirection _direction
        (:Forward
          (CallFunction|MovingBackward))
        (:Backward
          (CallFunction|MovingForward))))))

(event EventBeginPlay
  ;[1 1 1] Startup
  (Utilities|FlowControl|Sequence
    (:then_1
      ;[1 1 1] Set Playrate
      (Components|Timeline|SetPlayRate (Variables|Default|GetPatrolTimeline) (/ 1.0 (Variables|Default|GetpatrolSpeed)))
      (Variables|Default|SettestRightEnd true))))

(fn ConstructionScript
  (Transformation|SetRelativeLocation (Variables|Default|GetMovingPlatform) (Math|Vector|SelectVector (Variables|Default|GetrightEndPoint) "0, 0, 0" (Variables|Default|GettestRightEnd)) false false))