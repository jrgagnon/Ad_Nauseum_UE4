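; Breakable wall actor, filed under traps, that bullets can destroy.
; It copies MaxHealth into CurrentHealth on BeginPlay.
; Each overlap with a BulletGeneral actor subtracts that bullet's Damage from CurrentHealth, and the wall destroys itself once health reaches zero or below.
; Damage is read directly from the overlapping bullet through a cast, and other actors are ignored.
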(event Collision|EventActorBeginOverlap
  (params (OtherActor :type Actor%20Object%20Reference))
  (bind _asbullet_general (Utilities|Casting|CastToBulletGeneral OtherActor))
  (bind _output_get (Variables|Default|SetcurrentHealth (- (Variables|Default|GetcurrentHealth) (Variables|/Game/Ad_Nauseum/Blueprints/General/BulletGeneral.BulletGeneral_C|Getdamage _asbullet_general))))
  (if (<= _output_get 0.0)
    (Actor|DestroyActor)))

(event EventBeginPlay
  (Variables|Default|SetcurrentHealth (Variables|Default|GetmaxHealth)))

(fn ConstructionScript)