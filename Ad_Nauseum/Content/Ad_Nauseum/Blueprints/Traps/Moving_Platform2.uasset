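; Moving platform trap that travels one way from its origin to RightEndPoint, then replaces itself with a fresh copy.
; MovingForward plays a timeline that lerps the platform's relative location, with play rate set at BeginPlay as the inverse of PatrolSpeed.
; On finish it spawns a new instance with the same endpoint and destroys only its platform component, not the actor.
; The construction script uses TestRightEnd to place the platform at either end.
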(event Custom|Moving%20Forward
  ;[1 1 1] Movement Control
  (bind _driver (Timeline|PatrolTimeline PlayFromStart)
    (:Update
      (Transformation|SetRelativeLocation (Variables|Default|GetMovingPlatform) (Math|Vector|Lerp(Vector) "0, 0, 0" (Variables|Default|GetrightEndPoint) _driver) false false))
    (:Finished
      (bind _returnvalue (Game|SpawnActorfromClass "Moving_Platform2_C" (Transformation|GetActorTransform (Components|GetOwner (Variables|Default|GetMovingPlatform))) "Undefined" 0 0))
      (Variables|Moving_Platform2_C|SetrightEndPoint _returnvalue (Variables|Default|GetrightEndPoint))
      (Components|DestroyComponent (Variables|Default|GetMovingPlatform)))))

(event EventBeginPlay
  ;[1 1 1] Startup
  (Utilities|FlowControl|Sequence
    (:then_1
      ;[1 1 1] Set Playrate
      (Components|Timeline|SetPlayRate (Variables|Default|GetPatrolTimeline) (/ 1.0 (Variables|Default|GetpatrolSpeed)))
      (Variables|Default|SettestRightEnd true))))

(fn ConstructionScript
  (Transformation|SetRelativeLocation (Variables|Default|GetMovingPlatform) (Math|Vector|SelectVector (Variables|Default|GetrightEndPoint) "0, 0, 0" (Variables|Default|GettestRightEnd)) false false))