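; Top snowball of the snowman boss, which spawns the middle section on BeginPlay and turns its sprite toward the player.
; It interpolates to sit above the middle until that is gone, then enables gravity for a second phase; JumpMove supplies randomized hops toward the facing side.
; Player bullets reduce health and shrink it proportionally; it is destroyed at zero health, or on touching Slimey when tiny.
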(event OnComponentBeginOverlap(PaperSprite)
  (params (OverlappedComponent :type Primitive%20Component%20Object%20Reference) (OtherActor :type Actor%20Object%20Reference) (OtherComp :type Primitive%20Component%20Object%20Reference) (OtherBodyIndex :type Integer) (bFromSweep :type Boolean) (SweepResult :type Hit%20Result%20Structure%20%28by%20ref%29))
  ;[1 1 1] Actor Overlap Handling
  ;;[1 1 1] If Slimey is Hit Damage Him
  (Utilities|Casting|CastToSlimey OtherActor
    (:then
      (if (< (.x (Variables|Default|GetScale)) 0.1)
        (Actor|DestroyActor)))
    (:CastFailed
      ;;[1 1 1] If I am hit determine damage, then damage me
      (if (Utilities|ClassIsChildOf (Utilities|GetClass OtherActor) "/Game/Ad_Nauseum/Blueprints/General/BulletGeneral.BulletGeneral_C")
        (bind _asbullet_general (Utilities|Casting|CastToBulletGeneral OtherActor))
        (if (not (Variables|/Game/Ad_Nauseum/Blueprints/General/BulletGeneral.BulletGeneral_C|GetenemyBullet _asbullet_general))
          (CallFunction|PatrolHit (Variables|/Game/Ad_Nauseum/Blueprints/General/BulletGeneral.BulletGeneral_C|Getdamage _asbullet_general)))))))

(event Custom|Jump%20Move
  (bind _returnvalue (Math|Random|RandomFloatinRange 0.6 1.0))
  (bind _bossjumpforce (Variables|Default|GetBossJumpForce))
  (bind _returnvalue_2 (* _bossjumpforce _returnvalue))
  (if (Variables|Default|GetFacing)
    (Physics|AddForce (Variables|Default|GetPaperSprite) (Math|Vector|MakeVector (/ _returnvalue_2 2.0) 0.0 _bossjumpforce) "None" false)
    (else
      (Physics|AddForce (Variables|Default|GetPaperSprite) (Math|Vector|MakeVector (/ _returnvalue_2 -2.0) 0.0 _bossjumpforce) "None" false))))

(event Custom|PatrolHit
  (params (DamageIn :type Float%20%28single-precision%29))
  (bind _returnvalue (Transformation|GetActorTransform))
  (bind _currenthealth (Variables|Default|GetCurrentHealth))
  (bind _maxhealth (Variables|Default|GetMaxHealth))
  (bind _returnvalue_2 (/ _currenthealth _maxhealth))
  (bind _returnvalue_3 (* _returnvalue_2 0.4))
  ;[1 1 1] Damage Me
  (Utilities|FlowControl|Sequence
    (:then_0
      (bind _output_get (Variables|Default|SetcurrentHealth (- (Variables|Default|GetcurrentHealth) DamageIn)))
      ;[1 1 1] Kill me if health is <= 0
      (if (<= _output_get 0.0)
        (Actor|DestroyActor)))
    (:then_1
      (Variables|Default|SetScale (Math|Vector|MakeVector _returnvalue_3 _returnvalue_3 _returnvalue_3))
      (Transformation|SetActorTransform (Math|Transform|MakeTransform (.location _returnvalue) (.rotation _returnvalue) (Variables|Default|GetScale))))))

(event EventBeginPlay
  (bind _returnvalue (Transformation|GetActorLocation))
  ;[1 1 1] On Startup
  (bind _returnvalue_2 (Game|SpawnActorfromClass "/Game/Ad_Nauseum/Blueprints/BasicMobs/SnowmanBossMiddle.SnowmanBossMiddle_C" (Math|Transform|MakeTransform (Math|Vector|MakeVector (.x _returnvalue) (.y _returnvalue) (- (.z _returnvalue) 1e+02)) "0, 0,0.000000" "0.600000,0.600000,0.600000") "Undefined" 0 0))
  (Variables|Default|SetMiddle _returnvalue_2)
  (Variables|Default|SetCurrentHealth (Variables|Default|GetMaxHealth)))

(event Collision|EventActorBeginOverlap
  (params (OtherActor :type Actor%20Object%20Reference)))

(event EventTick
  (params (DeltaSeconds :type Float%20%28single-precision%29))
  (bind _returnvalue (Transformation|GetActorLocation))
  (bind _middle (Variables|Default|GetMiddle))
  (bind _returnvalue_2 (Transformation|GetActorLocation _middle))
  (bind _returnvalue_3 (+ (.z _returnvalue_2) 2.5e+02))
  (bind _returnvalue_4 (Class|KismetMathLibrary|Vector2DInterpto (Math|Vector2D|MakeVector2D (.x _returnvalue) (.z _returnvalue)) (Math|Vector2D|MakeVector2D (.x _returnvalue_2) _returnvalue_3) DeltaSeconds 1e+01))
  (Utilities|FlowControl|Sequence
    (:then_0
      ;[1 1 1] Set middle section facing
      (if (< (.x (Transformation|GetActorLocation (Game|Player|GetPlayerPawn 0))) (.x (Transformation|GetActorLocation)))
        (Variables|Default|SetFacing false)
        (else
          (Variables|Default|SetFacing true))))
    (:then_1
      (bind _returnvalue_5 (Physics|GetPhysicsLinearVelocity (Variables|Default|GetPaperSprite) "None"))
      (if (Variables|Default|GetFacing)
        (Rendering|Components|Sprite|SetSprite (Variables|Default|GetPaperSprite) "/Game/Ad_Nauseum/Sprites/RightFacingTopSnowball_Sprite.RightFacingTopSnowball_Sprite")
        (Physics|SetPhysicsLinearVelocity (Variables|Default|GetPaperSprite) _returnvalue_5 false "None")
        (else
          (Rendering|Components|Sprite|SetSprite (Variables|Default|GetPaperSprite) "/Game/Ad_Nauseum/Sprites/LeftFacingTopSnowball_Sprite.LeftFacingTopSnowball_Sprite")
          (Physics|SetPhysicsLinearVelocity (Variables|Default|GetPaperSprite) _returnvalue_5 false "None"))))
    (:then_3
      ;[1 1 1] Second Phase
      (if (Variables|Default|GetBottomDead)
        (if (Variables|Default|GetDumbbool)
          (Utilities|FlowControl|Sequence
            (:then_0
              (Physics|SetEnableGravity (Variables|Default|GetPaperSprite) true))
            (:then_1
              (Variables|Default|SetDumbbool false))))
        (else
          (Utilities|IsValid (Variables|Default|GetMiddle)
            (:Is%20Valid
              ;[1 1 1] Interp
              (Transformation|SetActorLocation (Math|Vector|MakeVector (.x _returnvalue_4) 0.0 (.y _returnvalue_4)) false false))
            (:Is%20Not%20Valid
              (Variables|Default|SetBottomDead true))))))))

(fn ConstructionScript)