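; YellowSlime is a basic mob that patrols back and forth along the X axis between Leftpost and Rightpost.
; A timeline interpolates its location, playing forward or in reverse according to the Boobian flag.
; When the timeline finishes, it toggles the flag, mirrors the actor by negating X scale and restarts the movement event.
; BeginPlay starts the patrol and, after a delay, spawns a Justthebutt actor at a fixed location.
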(event Custom|CustomEvent_0
  (bind _returnvalue (Transformation|GetActorTransform))
  (bind _returnvalue_2 (Transformation|GetActorLocation))
  (bind _leftpost (Variables|Default|GetLeftpost))
  (if (Variables|Default|Getboobian)
    (bind _newtrack_0 (Timeline|Timeline_0 PlayFromStart)
      (:Update
        (Transformation|SetActorLocation (Math|Vector|MakeVector (+ _leftpost (* _newtrack_0 (- (Variables|Default|GetRightpost) _leftpost))) (.y _returnvalue_2) (.z _returnvalue_2)) false false))
      (:Finished
        (Variables|Default|Setboobian (not (Variables|Default|Getboobian)))
        (Transformation|SetActorTransform (Math|Transform|MakeTransform (.location _returnvalue) (.rotation _returnvalue) (Math|Vector|MakeVector (* (.x (.scale _returnvalue)) -1.0) (.y (.scale _returnvalue)) (.z (.scale _returnvalue)))))
        (CallFunction|CustomEvent0)))
    (else
      (Timeline|Timeline_0 ReverseFromEnd))))

(event EventBeginPlay
  (Utilities|FlowControl|Sequence
    (:then_0
      (CallFunction|CustomEvent0))
    (:then_1
      (Utilities|FlowControl|Delay 2e+01)
      (Game|SpawnActorfromClass "/Game/Ad_Nauseum/Blueprints/BasicMobs/Justthebutt.Justthebutt_C" (Math|Transform|MakeTransform "662.000000, 0,1080.000000" "0, 0, 0" "1,1,1") "Undefined" 0 0))))

(event Collision|EventActorBeginOverlap
  (params (OtherActor :type Actor%20Object%20Reference)))

(event EventTick
  (params (DeltaSeconds :type Float%20%28single-precision%29)))

(fn ConstructionScript)